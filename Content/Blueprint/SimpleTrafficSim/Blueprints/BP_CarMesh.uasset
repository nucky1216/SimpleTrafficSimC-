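; Vehicle actor for the simple traffic simulation, with driving delegated to its BPCSimMovement component.
; Construction sets the mesh by CarType, fits CarBox to its bounds, parses CarID from the display name and configures auto-drive.
; An optional debug widget, colored by ID, shows speeds every tick.
; Events swap car and cube meshes, draw or rebuild detection boxes, test lane switching and relay the component's destroyed notification.
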(event Custom|Autobots
  (params (Autobot :type Boolean))
  (bind _staticmesh (Variables|Default|GetStaticMesh))
  (if (!= Autobot (Variables|Default|GetAutobot))
    (if Autobot
      (Components|StaticMesh|SetStaticMesh _staticmesh (Utilities|Array|Get(acopy) (Variables|Default|GetCarMeshes) (Variables|Default|GetCarType)))
      (Variables|Default|SetAutobot true)
      (else
        (Components|StaticMesh|SetStaticMesh _staticmesh "/SimpleTrafficSim/Blueprint/SimpleTrafficSim/Car_Mesh/Mesh/SM_CubeCar.SM_CubeCar")
        (Variables|Default|SetAutobot false)))))

(event Custom|ShowBox
  (Default|DrawCarBox (Variables|Default|GetBPC_SimMovement) 1e+01))

(event Custom|Debug
  (Utilities|FlowControl|Sequence
    (:then_0
      (for _array_element (Actor|GetComponentsbyTag "/Script/Engine.BoxComponent" "ForwardBox")
        (Components|DestroyComponent _array_element)))
    (:then_1
      (Default|AddForwardDetectBox (Variables|Default|GetBPC_SimMovement)))))

(event Custom|TestSwitch
  (Variables|/SimpleTrafficSim/Blueprint/SimpleTrafficSim/Blueprints/BPC_SimMovement.BPC_SimMovement_C|SetSpline (Variables|Default|GetBPC_SimMovement) (Variables|/SimpleTrafficSim/Blueprint/SimpleTrafficSim/Blueprints/RoadSpline/BP_SplineLane.BP_SplineLane_C|GetSpline (Variables|Default|GetLane)))
  (Default|SwithLane (Variables|Default|GetBPC_SimMovement)))

(event EventBeginPlay
  (EventDispatchers|BindEventtoVehicleHasDestroyed (Variables|Default|GetBPC_SimMovement) (EventDispatchers|CreateEvent :!event VehicleHasDestroyed))
  (if (Variables|Default|GetDebugWidget)
    (bind _asui_car_infor (Utilities|Casting|CastToUI_CarInfor (UserInterface|GetUserWidgetObject (Variables|Default|GetWidget))))
    (Variables|Default|SetUI_CarInfor _asui_car_infor)
    (Default|SetColor (Variables|Default|GetUI_CarInfor) (Variables|Default|GetCarID))))

(event EventTick
  (params (DeltaSeconds :type Float%20%28single-precision%29))
  (bind _bpc_simmovement (Variables|Default|GetBPC_SimMovement))
  (if (Variables|Default|GetDebugWidget)
    (Default|SetInfor (Variables|Default|GetUI_CarInfor) (Utilities|Text|FormatText "  S:{Speed}  
ES:{ExpSpeed} 
MS:{MaxSpeed}" (Utilities|Text|ToText(Float) (Variables|/SimpleTrafficSim/Blueprint/SimpleTrafficSim/Blueprints/BPC_SimMovement.BPC_SimMovement_C|GetSpeed _bpc_simmovement) "HalfToEven" false false 3 4 2 2) (Utilities|Text|ToText(Float) (Variables|/SimpleTrafficSim/Blueprint/SimpleTrafficSim/Blueprints/BPC_SimMovement.BPC_SimMovement_C|GetExpectSpeed _bpc_simmovement) "HalfToEven" false false 3 4 2 2) (Utilities|Text|ToText(Float) (Variables|/SimpleTrafficSim/Blueprint/SimpleTrafficSim/Blueprints/BPC_SimMovement.BPC_SimMovement_C|GetMaxSpeed _bpc_simmovement) "HalfToEven" false false 3 4 2 2)))))

(fn ConstructionScript
  (bind _self self)
  (bind _carmeshes (Variables|Default|GetCarMeshes))
  (bind _widget (Variables|Default|GetWidget))
  (bind _cartype (Variables|Default|GetCarType))
  (bind _bpc_simmovement (Variables|Default|GetBPC_SimMovement))
  (bind _returnvalue (Utilities|GetDisplayName _self))
  (bind _output (Utilities|Array|Get(acopy) _carmeshes _cartype))
  (bind _rights (Utilities|String|Split _returnvalue "BP_CarMesh" "IgnoreCase" "FromEnd"))
  (bind _returnvalue_2 (Math|Conversions|ToInteger(Byte) _rights))
  (Components|StaticMesh|SetStaticMesh (Variables|Default|GetStaticMesh) _output)
  (CallFunction|BoxTransform _output)
  (Variables|Default|SetCarID _returnvalue_2)
  (Default|ConfigAutoDriveParms (Variables|Default|GetBPC_SimMovement) (Variables|Default|GetAuto%20Drive) (Variables|Default|GetCarBox) 0.0 0.0 (Variables|Default|GetNext%20Lane) _returnvalue_2)
  (if (Variables|Default|GetDebugWidget)
    (bind _asui_car_infor (Utilities|Casting|CastToUI_CarInfor (UserInterface|GetWidget _widget)))
    (Variables|Default|SetUI_CarInfor _asui_car_infor)
    (Default|SetInfor (Variables|Default|GetUI_CarInfor) (Utilities|Text|FormatText "S:{Speed} ES:{ExpSpeed}" (Utilities|Text|ToText(Float) (Variables|/SimpleTrafficSim/Blueprint/SimpleTrafficSim/Blueprints/BPC_SimMovement.BPC_SimMovement_C|GetSpeed _bpc_simmovement) "HalfToEven" false true 3 4 2 2) (Utilities|Text|ToText(Float) (Variables|/SimpleTrafficSim/Blueprint/SimpleTrafficSim/Blueprints/BPC_SimMovement.BPC_SimMovement_C|GetExpectSpeed _bpc_simmovement) "HalfToEven" false true 3 4 2 2)))
    (Default|SetColor (Variables|Default|GetUI_CarInfor) _returnvalue_2)
    (else
      (Rendering|SetVisibility _widget false false))))

(fn BoxTransform
  (params (StaticMesh :type Static%20Mesh%20Object%20Reference))
  (bind _returnvalue (StaticMesh|GetBoundingBox StaticMesh))
  (bind _carbox (Variables|Default|GetCarBox))
  (bind (_min _max) (Utilities|Struct|BreakBox _returnvalue))
  (bind _returnvalue_2 (- _max _min))
  (Transformation|SetWorldScale3D _carbox (/ _returnvalue_2 1e+02))
  (Transformation|SetRelativeLocation _carbox (* _returnvalue_2 "0.000000,0.000000,0.500000") false false))

(fn VehicleHasDestroyed
  (Default|CallNotifyVehicleHasDestroyed))