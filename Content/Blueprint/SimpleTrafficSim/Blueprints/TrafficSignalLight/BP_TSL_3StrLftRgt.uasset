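; Traffic signal light variant for the traffic sim, apparently straight/left/right, that adds a right-side red, yellow and green light set to its parent.
; Its Create Light Mesh Mat Instance override calls the parent, then creates and stores a colored dynamic instance of MI_SignalTest for each right lamp.
; Green and yellow start with zero emissive, while red keeps the material's value.
; The event graph and construction script add no logic of their own.
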(event EventBeginPlay
  (|CallParentFunction) ; This node is disabled and will not be called.\nDrag off pins to build functionality.
)

(event Collision|EventActorBeginOverlap
  (params (OtherActor :type Actor%20Object%20Reference))
  (|CallParentFunction OtherActor) ; This node is disabled and will not be called.\nDrag off pins to build functionality.
)

(event EventTick
  (params (DeltaSeconds :type Float%20%28single-precision%29))
  (|CallParentFunction DeltaSeconds) ; This node is disabled and will not be called.\nDrag off pins to build functionality.
)

(fn ConstructionScript
  (|CallParentFunction))

(fn CreateLightMeshMatInstance
  (|CallParentFunction)
  (Utilities|FlowControl|Sequence
    (:then_0
      (bind _returnvalue (Rendering|Material|CreateDynamicMaterialInstance "/SimpleTrafficSim/Blueprint/SimpleTrafficSim/Blueprints/DebugMaterial/MI_SignalTest.MI_SignalTest" "None" "None" :!class /Script/Engine.KismetMaterialLibrary))
      (bind _output_get (Variables|Default|SetMatRightGreenLight _returnvalue))
      (Rendering|Material|SetMaterial (Variables|Default|GetRightGreen) 0 _output_get)
      (Rendering|Material|SetVectorParameterValue _output_get "Color" "(R=0.000000,G=1.000000,B=0.000000,A=1.000000)" :!class /Script/Engine.MaterialInstanceDynamic)
      (Rendering|Material|SetScalarParameterValue _output_get "Emissive" 0.0 :!class /Script/Engine.MaterialInstanceDynamic))
    (:then_1
      (bind _returnvalue_2 (Rendering|Material|CreateDynamicMaterialInstance "/SimpleTrafficSim/Blueprint/SimpleTrafficSim/Blueprints/DebugMaterial/MI_SignalTest.MI_SignalTest" "None" "None" :!class /Script/Engine.KismetMaterialLibrary))
      (bind _output_get_2 (Variables|Default|SetMatRightYellowLight _returnvalue_2))
      (Rendering|Material|SetMaterial (Variables|Default|GetRightYellow) 0 _output_get_2)
      (Rendering|Material|SetVectorParameterValue _output_get_2 "Color" "(R=1.000000,G=1.000000,B=0.000000,A=1.000000)" :!class /Script/Engine.MaterialInstanceDynamic)
      (Rendering|Material|SetScalarParameterValue _output_get_2 "Emissive" 0.0 :!class /Script/Engine.MaterialInstanceDynamic))
    (:then_2
      (bind _returnvalue_3 (Rendering|Material|CreateDynamicMaterialInstance "/SimpleTrafficSim/Blueprint/SimpleTrafficSim/Blueprints/DebugMaterial/MI_SignalTest.MI_SignalTest" "None" "None" :!class /Script/Engine.KismetMaterialLibrary))
      (bind _output_get_3 (Variables|Default|SetMatRightRedLight _returnvalue_3))
      (Rendering|Material|SetMaterial (Variables|Default|GetRightRed) 0 _output_get_3)
      (Rendering|Material|SetVectorParameterValue _output_get_3 "Color" "(R=1.000000,G=0.000000,B=0.000000,A=1.000000)" :!class /Script/Engine.MaterialInstanceDynamic))))