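; Traffic signal actor for the simple traffic sim, with green, yellow and red lights for straight-ahead traffic.
; The construction script builds dynamic materials for the three lamp meshes and a debug board, then hands the lamp materials to BPCTrafficSignalLight.
; One second after BeginPlay, the board shows the component's light group as a number texture, or an error icon when none is assigned.
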(event EventBeginPlay
  (Utilities|FlowControl|Delay 1.0)
  (Rendering|Material|SetTextureParameterValue (Variables|Default|GetDebugPlaneBoard) "Texture" (Utilities|Select :Index (Variables|/SimpleTrafficSim/Blueprint/SimpleTrafficSim/Blueprints/TrafficSignalLight/BPC_TrafficSignalLight.BPC_TrafficSignalLight_C|GetLightGroup (Variables|Default|GetBPC_TrafficSignalLight)) :NewEnumerator2 "/Dimensio/MaterialDesignUI/Components/Image/Notification/Notification_Icon_Error_Outline.Notification_Icon_Error_Outline" :NewEnumerator0 "/SimpleTrafficSim/Blueprint/SimpleTrafficSim/Blueprints/DebugMaterial/T_Number1.T_Number1" :NewEnumerator1 "/SimpleTrafficSim/Blueprint/SimpleTrafficSim/Blueprints/DebugMaterial/T_Number2.T_Number2")))

(fn ConstructionScript
  (Utilities|FlowControl|Sequence
    (:then_0
      (bind _returnvalue (Rendering|Material|CreateDynamicMaterialInstance "/SimpleTrafficSim/Blueprint/SimpleTrafficSim/Blueprints/DebugMaterial/MI_TextureMaterial.MI_TextureMaterial" "None" "None" :!class /Script/Engine.KismetMaterialLibrary))
      (bind _output_get (Variables|Default|SetDebugPlaneBoard _returnvalue))
      (Rendering|Material|SetMaterial (Variables|Default|GetPlane) 0 _output_get))
    (:then_1
      (CallFunction|CreateLightMeshMatInstance)
      (CallFunction|PassMaterial2TSLComponent))))

(fn CreateLightMeshMatInstance
  (Utilities|FlowControl|Sequence
    (:then_0
      (bind _returnvalue (Rendering|Material|CreateDynamicMaterialInstance "/SimpleTrafficSim/Blueprint/SimpleTrafficSim/Blueprints/DebugMaterial/MI_SignalTest.MI_SignalTest" "None" "None" :!class /Script/Engine.KismetMaterialLibrary))
      (bind _output_get (Variables|Straight|SetMatGreenLight _returnvalue))
      (Rendering|Material|SetMaterial (Variables|Default|GetGreen) 0 _output_get)
      (Rendering|Material|SetVectorParameterValue _output_get "Color" "(R=0.000000,G=1.000000,B=0.000000,A=1.000000)" :!class /Script/Engine.MaterialInstanceDynamic)
      (Rendering|Material|SetScalarParameterValue _output_get "Emissive" 0.0 :!class /Script/Engine.MaterialInstanceDynamic))
    (:then_1
      (bind _returnvalue_2 (Rendering|Material|CreateDynamicMaterialInstance "/SimpleTrafficSim/Blueprint/SimpleTrafficSim/Blueprints/DebugMaterial/MI_SignalTest.MI_SignalTest" "None" "None" :!class /Script/Engine.KismetMaterialLibrary))
      (bind _output_get_2 (Variables|Straight|SetMatYellowLight _returnvalue_2))
      (Rendering|Material|SetMaterial (Variables|Default|GetYellow) 0 _output_get_2)
      (Rendering|Material|SetVectorParameterValue _output_get_2 "Color" "(R=1.000000,G=1.000000,B=0.000000,A=1.000000)" :!class /Script/Engine.MaterialInstanceDynamic)
      (Rendering|Material|SetScalarParameterValue _output_get_2 "Emissive" 0.0 :!class /Script/Engine.MaterialInstanceDynamic))
    (:then_2
      (bind _returnvalue_3 (Rendering|Material|CreateDynamicMaterialInstance "/SimpleTrafficSim/Blueprint/SimpleTrafficSim/Blueprints/DebugMaterial/MI_SignalTest.MI_SignalTest" "None" "None" :!class /Script/Engine.KismetMaterialLibrary))
      (bind _output_get_3 (Variables|Straight|SetMatRedLight _returnvalue_3))
      (Rendering|Material|SetMaterial (Variables|Default|GetRed) 0 _output_get_3)
      (Rendering|Material|SetVectorParameterValue _output_get_3 "Color" "(R=1.000000,G=0.000000,B=0.000000,A=1.000000)" :!class /Script/Engine.MaterialInstanceDynamic))))

(fn PassMaterial2TSLComponent
  (Default|GetLightMat (Variables|Default|GetBPC_TrafficSignalLight) (Variables|Straight|GetMatGreenLight) (Variables|Straight|GetMatYellowLight) (Variables|Straight|GetMatRedLight) (Variables|Left|GetMatLeftGreenLight) (Variables|Left|GetMatLeftYellowLight) (Variables|Left|GetMatLeftRedLight) (Variables|Right|GetMatRightGreenLight) (Variables|Right|GetMatRightYellowLight) (Variables|Right|GetMatRightRedLight) "Albedo TInt"))