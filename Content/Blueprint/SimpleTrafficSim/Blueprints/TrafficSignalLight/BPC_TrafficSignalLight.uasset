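; Traffic signal light component that switches its owner's red, yellow and green lamps to follow a road crossing's signal cycle.
; On BeginPlay it binds to the first crossroad BP_RoadConnector within range and can auto-pick its light group from the nearest TLSPosition.
; Assigned materials determine the head type: straight, plus optional left and right arrows.
; Crossing change events drive scalar material parameters per lamp, filtered by visibility and light group.
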(event EventBeginPlay
  (bind _roadcross (Variables|Default|GetRoadCross))
  (Utilities|FlowControl|Delay 0.2)
  (CallFunction|FindNeibourCross 5.5e+03)
  (Utilities|IsValid _roadcross
    (:Is%20Valid
      (if (Variables|Default|GetAutoBind)
        (CallFunction|FindLightGroup))
      (EventDispatchers|BindEventtoTSLChange _roadcross (EventDispatchers|CreateEvent :!event TrafficSignalLightChange))
      (Variables|Default|SetTSLType (CallFunction|GetTSLType)))))

(event EventTick
  (params (DeltaSeconds :type Float%20%28single-precision%29)))

(fn FindNeibourCross
  (params (Radius :type Float%20%28double-precision%29))
  (Utilities|IsValid (Variables|Default|GetRoadCross)
    (:Is%20Not%20Valid
      (bind _outactors (Actor|GetAllActorsOfClass "/SimpleTrafficSim/Blueprint/SimpleTrafficSim/Blueprints/RoadSpline/BP_RoadConnector.BP_RoadConnector_C"))
      (LocalVariables|SetFinded false)
      (bind _array_element (Utilities|Array|ForEachLoopwithBreak _outactors :!label _label)
        (:LoopBody
          (if (not (Variables|/SimpleTrafficSim/Blueprint/SimpleTrafficSim/Blueprints/RoadSpline/BP_RoadConnector.BP_RoadConnector_C|GetNot%20Cross%20Road _array_element))
            (if (<= (Math|Vector|Distance(Vector) (Transformation|GetActorLocation _array_element) (Transformation|GetActorLocation (Components|GetOwner))) Radius)
              (Variables|Default|SetRoadCross _array_element)
              (LocalVariables|SetFinded true)
              (goto _label Break))))
        (:Completed
          (if (LocalVariables|GetFinded)
            (Class|DimensioBPLibrary|PrintLog (Utilities|String|Append (Utilities|GetDisplayName (Components|GetOwner)) " has bind to " (Utilities|GetDisplayName (Variables|Default|GetRoadCross))))
            (else
              (Class|DimensioBPLibrary|PrintLog (Utilities|String|Append "Cannot Bind to NeiborCross with radius:" (Utilities|String|ToString(Float) Radius)) true true "(R=0.000000,G=0.660000,B=1.000000,A=1.000000)" 2.0 "Warning"))))))))

(fn TrafficSignalLightChange
  (params (LightSignal :type E_LightState%20Enum :default "NewEnumerator0") (LightGroupType :type E_LightsGroupType%20Enum :default "NewEnumerator0"))
  (if (Variables|/Script/Engine.SceneComponent|GetbVisible (Actor|GetComponentbyClass (Components|GetOwner) "/Script/Engine.SceneComponent"))
    (if (Utilities|IsinCurLightGroup (Variables|Default|GetLightGroup) LightGroupType)
      (switch Utilities|FlowControl|Switch|SwitchonE_TSLType (Variables|Default|GetTSLType)
        (:NewEnumerator0
          (CallFunction|LightonStr LightSignal LightGroupType))
        (:NewEnumerator1
          (CallFunction|LightonStr&Left LightSignal LightGroupType))
        (:NewEnumerator2
          (CallFunction|LightonStr&Left&Right LightSignal LightGroupType))
        (:NewEnumerator3
          (Class|DimensioBPLibrary|PrintLog (Utilities|String|Append "Failed Get Light Materials from Cross:" (Utilities|GetDisplayName (Components|GetOwner))) true true "(R=0.000000,G=0.660000,B=1.000000,A=1.000000)" 2.0 "Warning"))))))

(fn LightonStr&Left
  (params (Signal :type E_LightState%20Enum :default "NewEnumerator0") (LightType :type E_LightsGroupType%20Enum :default "NewEnumerator0"))
  (bind _lightgroup (Variables|Default|GetLightGroup))
  (bind _returnvalue (Utilities|Select :Index _lightgroup :NewEnumerator2 "NewEnumerator0" :NewEnumerator0 "NewEnumerator4" :NewEnumerator1 "NewEnumerator5"))
  (bind _returnvalue_2 (Utilities|Enum|Equal(Enum) LightType _returnvalue))
  (bind _returnvalue_3 (not _returnvalue_2))
  (Utilities|FlowControl|Sequence
    (:then_0
      (CallFunction|LightonOff (Variables|Default|GetS_GreenMat) "NewEnumerator1" (and (Utilities|Enum|Equal(Enum) "NewEnumerator2" Signal) _returnvalue_3))
      (CallFunction|LightonOff (Variables|Default|GetS_YellowMat) "NewEnumerator2" (and (Utilities|Enum|Equal(Enum) "NewEnumerator1" Signal) _returnvalue_3))
      (CallFunction|LightonOff (Variables|Default|GetS_RedMat) "NewEnumerator0" (or (Utilities|Enum|Equal(Enum) "NewEnumerator0" Signal) (not _returnvalue_3))))
    (:then_1
      (CallFunction|LightonOff (Variables|Default|GetL_GreenMat) "NewEnumerator1" (and (Utilities|Enum|Equal(Enum) Signal "NewEnumerator2") _returnvalue_2))
      (CallFunction|LightonOff (Variables|Default|GetL_YellowMat) "NewEnumerator2" (and (Utilities|Enum|Equal(Enum) Signal "NewEnumerator1") _returnvalue_2))
      (CallFunction|LightonOff (Variables|Default|GetL_RedMat) "NewEnumerator0" (or (Utilities|Enum|Equal(Enum) Signal "NewEnumerator0") (not _returnvalue_2))))))

(fn GetLightMat
  (params (StraightGreen :type Material%20Instance%20Dynamic%20Object%20Reference) (StraightYellow :type Material%20Instance%20Dynamic%20Object%20Reference) (StraightRed :type Material%20Instance%20Dynamic%20Object%20Reference) (LeftGreen :type Material%20Instance%20Dynamic%20Object%20Reference) (LeftYellow :type Material%20Instance%20Dynamic%20Object%20Reference) (LeftRed :type Material%20Instance%20Dynamic%20Object%20Reference) (RightGreen :type Material%20Instance%20Dynamic%20Object%20Reference) (RightYellow :type Material%20Instance%20Dynamic%20Object%20Reference) (RightRed :type Material%20Instance%20Dynamic%20Object%20Reference) (Mat%20Clolor%20Param%20Name :type Name :default "Albedo TInt"))
  (Variables|Default|SetS_GreenMat StraightGreen)
  (Variables|Default|SetS_YellowMat StraightYellow)
  (Variables|Default|SetS_RedMat StraightRed)
  (Variables|Default|SetL_GreenMat LeftGreen)
  (Variables|Default|SetL_YellowMat LeftYellow)
  (Variables|Default|SetL_RedMat LeftRed)
  (Variables|Default|SetR_GreenMat RightGreen)
  (Variables|Default|SetR_YellowMat RightYellow)
  (Variables|Default|SetR_RedMat RightRed)
  (Variables|Default|SetMatParamName Mat%20Clolor%20Param%20Name))

(fn LightonStr
  (params (Signal :type E_LightState%20Enum :default "NewEnumerator0") (LightType :type E_LightsGroupType%20Enum :default "NewEnumerator0"))
  (bind _lightgroup (Variables|Default|GetLightGroup))
  (if (or (Utilities|Enum|Equal(Enum) LightType (Utilities|Select :Index _lightgroup :NewEnumerator2 "NewEnumerator0" :NewEnumerator0 "NewEnumerator0" :NewEnumerator1 "NewEnumerator1")) (Utilities|Enum|Equal(Enum) LightType (Utilities|Select :Index _lightgroup :NewEnumerator2 "NewEnumerator0" :NewEnumerator0 "NewEnumerator6" :NewEnumerator1 "NewEnumerator7")))
    (Utilities|FlowControl|Sequence
      (:then_0
        (CallFunction|LightonOff (Variables|Default|GetS_GreenMat) "NewEnumerator1" (Utilities|Enum|Equal(Enum) "NewEnumerator2" Signal))
        (CallFunction|LightonOff (Variables|Default|GetS_YellowMat) "NewEnumerator2" (Utilities|Enum|Equal(Enum) "NewEnumerator1" Signal))
        (CallFunction|LightonOff (Variables|Default|GetS_RedMat) "NewEnumerator0" (Utilities|Enum|Equal(Enum) "NewEnumerator0" Signal))))))

(fn GetTSLType
  (Utilities|FlowControl|Sequence
    (:then_0
      (if (Math|Boolean|ANDBoolean (Utilities|IsValid (Variables|Default|GetS_YellowMat)) (Utilities|IsValid (Variables|Default|GetS_GreenMat)) (Utilities|IsValid (Variables|Default|GetS_RedMat)))
        (if (Math|Boolean|ANDBoolean (Utilities|IsValid (Variables|Default|GetL_YellowMat)) (Utilities|IsValid (Variables|Default|GetL_GreenMat)) (Utilities|IsValid (Variables|Default|GetL_RedMat)))
          (if (Math|Boolean|ANDBoolean (Utilities|IsValid (Variables|Default|GetR_GreenMat)) (Utilities|IsValid (Variables|Default|GetR_YellowMat)) (Utilities|IsValid (Variables|Default|GetR_RedMat)))
            (return "NewEnumerator2")
            (else
              (return "NewEnumerator1")))
          (else
            (return "NewEnumerator0")))
        (else
          (return "NewEnumerator3"))))))

(fn LightonStr&Left&Right
  (params (Signal :type E_LightState%20Enum :default "NewEnumerator0") (LightType :type E_LightsGroupType%20Enum :default "NewEnumerator0"))
  (bind _lightgroup (Variables|Default|GetLightGroup))
  (bind _lightgroup_2 (Variables|Default|GetLightGroup))
  (bind _lightgroup_3 (Variables|Default|GetLightGroup))
  (bind _returnvalue (Utilities|Select :Index _lightgroup :NewEnumerator2 "NewEnumerator0" :NewEnumerator0 "NewEnumerator0" :NewEnumerator1 "NewEnumerator1"))
  (bind _returnvalue_2 (Utilities|Select :Index _lightgroup_2 :NewEnumerator2 "NewEnumerator0" :NewEnumerator0 "NewEnumerator4" :NewEnumerator1 "NewEnumerator4"))
  (bind _returnvalue_3 (Utilities|Select :Index _lightgroup_3 :NewEnumerator2 "NewEnumerator0" :NewEnumerator0 "NewEnumerator2" :NewEnumerator1 "NewEnumerator2"))
  (bind _returnvalue_4 (Utilities|Enum|Equal(Enum) LightType _returnvalue_2))
  (bind _returnvalue_5 (Utilities|Enum|Equal(Enum) LightType _returnvalue_3))
  (bind _returnvalue_6 (Utilities|Enum|Equal(Enum) LightType _returnvalue))
  (Utilities|FlowControl|Sequence
    (:then_0
      (Rendering|Material|SetScalarParameterValue (Variables|Default|GetS_GreenMat) "Emissive" (Math|Conversions|ToFloat(Boolean) (and (Utilities|Enum|Equal(Enum) "NewEnumerator2" Signal) _returnvalue_6)) :!class /Script/Engine.MaterialInstanceDynamic)
      (Rendering|Material|SetScalarParameterValue (Variables|Default|GetS_YellowMat) "Emissive" (Math|Conversions|ToFloat(Boolean) (and (Utilities|Enum|Equal(Enum) "NewEnumerator1" Signal) _returnvalue_6)) :!class /Script/Engine.MaterialInstanceDynamic)
      (Rendering|Material|SetScalarParameterValue (Variables|Default|GetS_RedMat) "Emissive" (Math|Conversions|ToFloat(Boolean) (or (Utilities|Enum|Equal(Enum) "NewEnumerator0" Signal) (not _returnvalue_6))) :!class /Script/Engine.MaterialInstanceDynamic))
    (:then_1
      (Rendering|Material|SetScalarParameterValue (Variables|Default|GetL_GreenMat) "Emissive" (Math|Conversions|ToFloat(Boolean) (and (Utilities|Enum|Equal(Enum) Signal "NewEnumerator2") _returnvalue_4)) :!class /Script/Engine.MaterialInstanceDynamic)
      (Rendering|Material|SetScalarParameterValue (Variables|Default|GetL_YellowMat) "Emissive" (Math|Conversions|ToFloat(Boolean) (and (Utilities|Enum|Equal(Enum) Signal "NewEnumerator1") _returnvalue_4)) :!class /Script/Engine.MaterialInstanceDynamic)
      (Rendering|Material|SetScalarParameterValue (Variables|Default|GetL_RedMat) "Emissive" (Math|Conversions|ToFloat(Boolean) (or (Utilities|Enum|Equal(Enum) Signal "NewEnumerator0") (not _returnvalue_4))) :!class /Script/Engine.MaterialInstanceDynamic))
    (:then_2
      (Rendering|Material|SetScalarParameterValue (Variables|Default|GetR_GreenMat) "Emissive" (Math|Conversions|ToFloat(Boolean) (and (Utilities|Enum|Equal(Enum) Signal "NewEnumerator2") _returnvalue_5)) :!class /Script/Engine.MaterialInstanceDynamic)
      (Rendering|Material|SetScalarParameterValue (Variables|Default|GetR_YellowMat) "Emissive" (Math|Conversions|ToFloat(Boolean) (and (Utilities|Enum|Equal(Enum) Signal "NewEnumerator1") _returnvalue_5)) :!class /Script/Engine.MaterialInstanceDynamic)
      (Rendering|Material|SetScalarParameterValue (Variables|Default|GetR_RedMat) "Emissive" (Math|Conversions|ToFloat(Boolean) (or (Utilities|Enum|Equal(Enum) Signal "NewEnumerator0") (not _returnvalue_5))) :!class /Script/Engine.MaterialInstanceDynamic))))

(fn FindLightGroup
  (bind _roadcross (Variables|Default|GetRoadCross))
  (bind _distance (LocalVariables|GetDistance))
  (bind _indexofminvalue (Math|Float|MinOfFloatArray _distance))
  (for _array_element (Variables|/SimpleTrafficSim/Blueprint/SimpleTrafficSim/Blueprints/RoadSpline/BP_RoadConnector.BP_RoadConnector_C|GetTLSPosition _roadcross)
    (Utilities|Array|Add (LocalVariables|GetDistance) (select (Utilities|Operators|NotEqual(!=) _array_element (Variables|/SimpleTrafficSim/Blueprint/SimpleTrafficSim/Blueprints/RoadSpline/BP_RoadConnector.BP_RoadConnector_C|GetInvalidPosiiton _roadcross) 0.0) (Math|Vector|Distance(Vector) _array_element (Transformation|GetActorLocation (Components|GetOwner))) (Math|Float|MakeLiteralFloat 999999999.0))))
  (bind _output_get (Variables|Default|SetLightGroup (Utilities|Select :Index _indexofminvalue :Option%200 "NewEnumerator0" :Option%201 "NewEnumerator0" :Option%202 "NewEnumerator1" :Option%203 "NewEnumerator1")))
  (Class|DimensioBPLibrary|PrintLog (Utilities|String|Append (Utilities|GetDisplayName (Components|GetOwner)) " has bind to " (Utilities|String|EnumtoString (Variables|Default|GetLightGroup)) " MinIdx:" (Utilities|String|ToString(Integer) _indexofminvalue)))
  (return _output_get))

(fn LightonOff
  (params (Mat :type Material%20Instance%20Dynamic%20Object%20Reference) (LightColor :type E_LightColor%20Enum :default "NewEnumerator0") (On :type Boolean))
  (Rendering|Material|SetScalarParameterValue Mat (Variables|Default|GetMatParamName) (Math|Float|SelectFloat 2.0 0.0 On) :!class /Script/Engine.MaterialInstanceDynamic))