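; BP_SImManager is the central manager of the simple traffic sim, building road splines and controlling the simulated cars.
; On construction and shortly after BeginPlay, it calls ConstructFunc on all road segments, then connectors; another event sticks segments to ground.
; Other events push tick and max-stop-time settings to SimCar-tagged movement components and spawners, cull cars by ReduceNum, and recount the total.
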(event Custom|Set%20Tick%20Counter
  (Utilities|FlowControl|FlipFlop
    (:A
      (bind _outactors (Actor|GetAllActorswithTag "SimCar"))
      (for _array_element _outactors
        (Variables|/SimpleTrafficSim/Blueprint/SimpleTrafficSim/Blueprints/BPC_SimMovement.BPC_SimMovement_C|SetLerpCounter (Actor|GetComponentbyClass _array_element "/SimpleTrafficSim/Blueprint/SimpleTrafficSim/Blueprints/BPC_SimMovement.BPC_SimMovement_C") (Variables|Default|GetTickCounter))))))

(event Custom|Set%20Max%20StopTime
  (Utilities|FlowControl|Sequence
    (:then_0
      (bind _outactors (Actor|GetAllActorswithTag "SimCar"))
      (for _array_element _outactors
        (Variables|/SimpleTrafficSim/Blueprint/SimpleTrafficSim/Blueprints/BPC_SimMovement.BPC_SimMovement_C|SetMaxStopTime (Actor|GetComponentbyClass _array_element "/SimpleTrafficSim/Blueprint/SimpleTrafficSim/Blueprints/BPC_SimMovement.BPC_SimMovement_C") (Variables|Default|GetMax%20Stop%20Time))))
    (:then_1
      (bind _outactors_2 (Actor|GetAllActorsOfClass "/SimpleTrafficSim/Blueprint/SimpleTrafficSim/Blueprints/BP_SpawnCar.BP_SpawnCar_C"))
      (for _array_element_2 _outactors_2
        (Variables|/SimpleTrafficSim/Blueprint/SimpleTrafficSim/Blueprints/BP_SpawnCar.BP_SpawnCar_C|SetMax%20Stop%20Time _array_element_2 (Variables|Default|GetMax%20Stop%20Time))))))

(event Custom|ReduceTheCarNumber
  (bind _outactors (Actor|GetAllActorswithTag "SimCar"))
  (bind _output_get (Variables|Default|SetCarMeshes _outactors))
  (Utilities|Array|Reverse _output_get)
  (Utilities|Array|Resize (Variables|Default|GetCarMeshes) (Variables|Default|GetReduceNum))
  (for _array_element (Variables|Default|GetCarMeshes)
    (Actor|DestroyActor _array_element))
  (bind _outactors_2 (Actor|GetAllActorswithTag "SimCar"))
  (Variables|Default|SetTotalNumber (Utilities|Array|Length _outactors_2)))

(event Custom|Get%20Total%20CarNumber
  (bind _outactors (Actor|GetAllActorswithTag "SimCar"))
  (Variables|Default|SetTotalNumber (Utilities|Array|Length _outactors)))

(event EventBeginPlay
  (|CallParentFunction)
  (Utilities|FlowControl|Delay 0.1)
  (CallFunction|ConstructSplines))

(event Collision|EventActorBeginOverlap
  (params (OtherActor :type Actor%20Object%20Reference))
  (|CallParentFunction OtherActor) ; This node is disabled and will not be called.\nDrag off pins to build functionality.
)

(event EventTick
  (params (DeltaSeconds :type Float%20%28single-precision%29))
  (|CallParentFunction DeltaSeconds) ; This node is disabled and will not be called.\nDrag off pins to build functionality.
)

(event Custom|Stick%20to%20Grount
  (Utilities|FlowControl|Sequence
    (:then_0
      (bind _outactors (Actor|GetAllActorsOfClass "/SimpleTrafficSim/Blueprint/SimpleTrafficSim/Blueprints/RoadSpline/BP_RoadSegment.BP_RoadSegment_C"))
      (for _array_element _outactors
        (Default|SticktoGround _array_element)))))

(event Custom|Construct%20Splines
  (Utilities|FlowControl|Sequence
    (:then_0
      (bind _outactors (Actor|GetAllActorsOfClass "/SimpleTrafficSim/Blueprint/SimpleTrafficSim/Blueprints/RoadSpline/BP_RoadSegment.BP_RoadSegment_C"))
      (for _array_element _outactors
        (Default|ConstructFunc _array_element)))
    (:then_1
      (bind _outactors_2 (Actor|GetAllActorsOfClass "/SimpleTrafficSim/Blueprint/SimpleTrafficSim/Blueprints/RoadSpline/BP_RoadConnector.BP_RoadConnector_C"))
      (for _array_element_2 _outactors_2
        (Default|ConstructFunc _array_element_2)))))

(fn ConstructionScript
  (|CallParentFunction)
  (CallFunction|ConstructSplines))