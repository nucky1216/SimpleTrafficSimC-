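; Road segment actor for the traffic sim that lays out parallel BP_SplineLane actors along a master spline.
; Construction offsets each lane by lane width, copies segment ID and light group to it, and positions end billboards.
; Events spawn or re-gather attached lanes, snap spline points to ground via line traces, and spawn a reversed-spline copy of the segment.
; A lookup finds adjacent lanes for lane switching.
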(event Custom|Get%20Attached%20Actors
  (CallFunction|GetAttachedLanes))

(event Custom|SpawnLanes
  (CallFunction|SpawnLanesbyNum (Variables|Road|GetLaneNum))
  (CallFunction|ConstructFunc))

(event Custom|Stick%20to%20Ground
  (CallFunction|TraceHeight (Variables|Default|GetHeight))
  (CallFunction|ConstructFunc))

(event Custom|MirroSegRoad
  (bind _spline (Variables|Default|GetSpline))
  (bind _returnvalue (Spline|GetNumberOfSplinePoints _spline))
  (bind _returnvalue_2 (- _returnvalue 1))
  (bind _returnvalue_3 (Spline|GetLocationatSplinePoint _spline _returnvalue_2 "World"))
  (bind _returnvalue_4 (Math|Conversions|ToTransform(Vector) _returnvalue_3))
  (bind _returnvalue_5 (Game|SpawnActorfromClass "BP_RoadSegment_C" _returnvalue_4 "Undefined" 0 0))
  (Variables|BP_RoadSegment_C|SetLaneNum _returnvalue_5 (Variables|Road|GetLaneNum))
  (Variables|BP_RoadSegment_C|SetHeight _returnvalue_5 (Variables|Default|GetHeight))
  (bind _splinelocalpoints (CallFunction|CopySpline (Math|Transform|InvertTransform _returnvalue_4)))
  (CallFunction|ApplySpline _returnvalue_5 _splinelocalpoints))

(event Custom|Draw%20LaneBox)

(event EventBeginPlay
  (|CallParentFunction))

(event Collision|EventActorBeginOverlap
  (params (OtherActor :type Actor%20Object%20Reference))
  (|CallParentFunction OtherActor) ; This node is disabled and will not be called.\nDrag off pins to build functionality.
)

(event EventTick
  (params (DeltaSeconds :type Float%20%28single-precision%29))
  (|CallParentFunction DeltaSeconds) ; This node is disabled and will not be called.\nDrag off pins to build functionality.
)

(fn ConstructionScript
  (|CallParentFunction)
  (CallFunction|ConstructFunc))

(fn LanePosition
  (bind _spline (Variables|Default|GetSpline))
  (bind _spline_2 (Variables|Default|GetSpline))
  (bind _lanes (Variables|Road|GetLanes))
  (bind _returnvalue (Spline|GetRotationatSplinePoint _spline 0 "World"))
  (bind _returnvalue_2 (Math|Vector|GetRightVector _returnvalue))
  (Variables|Default|SetSegID (Utilities|GetDisplayName self))
  (Variables|Input|SetlaneNumIn (Utilities|Array|Length _lanes))
  (for (_array_element _array_index) _lanes
    (Utilities|IsValid _array_element
      (:Is%20Valid
        (Variables|/SimpleTrafficSim/Blueprint/SimpleTrafficSim/Blueprints/RoadSpline/BP_SplineLane.BP_SplineLane_C|SetLaneID _array_element _array_index)
        (Variables|/SimpleTrafficSim/Blueprint/SimpleTrafficSim/Blueprints/RoadSpline/BP_SplineLane.BP_SplineLane_C|SetSegRef _array_element self)
        (Variables|/SimpleTrafficSim/Blueprint/SimpleTrafficSim/Blueprints/RoadSpline/BP_SplineLane.BP_SplineLane_C|SetSegID _array_element (Variables|Default|GetSegID))
        (Variables|/SimpleTrafficSim/Blueprint/SimpleTrafficSim/Blueprints/RoadSpline/BP_SplineLane.BP_SplineLane_C|SetLightGroup _array_element (Variables|Default|GetLightGroup))
        (Transformation|SetActorTransform _array_element (Math|Transform|MakeTransform (+ (* (* _array_index (Variables|Input|GetLaneWdith)) _returnvalue_2) (+ (Spline|GetLocationatSplinePoint _spline 0 "World") (* _returnvalue_2 -1.0 (* (Variables|Input|GetLaneWdith) (- (Math|Conversions|ToFloat(Integer) (/ (Variables|Input|GetlaneNumIn) 2)) 0.5))))) _returnvalue "1.000000,1.000000,1.000000"))
        (LocalVariables|SetCurSplinePointNum (Spline|GetNumberOfSplinePoints (Variables|/SimpleTrafficSim/Blueprint/SimpleTrafficSim/Blueprints/RoadSpline/BP_SplineLane.BP_SplineLane_C|GetSpline _array_element)))
        (for _index (range 0 (- (Spline|GetNumberOfSplinePoints _spline_2) 1))
          (if (>= _index (LocalVariables|GetCurSplinePointNum))
            (Spline|AddSplinePoint (Variables|/SimpleTrafficSim/Blueprint/SimpleTrafficSim/Blueprints/RoadSpline/BP_SplineLane.BP_SplineLane_C|GetSpline _array_element) (+ (* (* (Variables|Input|GetLaneWdith) _array_index) (Math|Vector|GetRightVector (Spline|GetRotationatSplinePoint _spline_2 _index "World"))) (+ (Spline|GetLocationatSplinePoint _spline_2 _index "World") (* (Math|Vector|GetRightVector (Spline|GetRotationatSplinePoint _spline_2 _index "World")) -1.0 (* (Variables|Input|GetLaneWdith) (- (Math|Conversions|ToFloat(Integer) (/ (Variables|Input|GetlaneNumIn) 2)) 0.5))))) "World" true)
            (else
              (Spline|SetLocationatSplinePoint (Variables|/SimpleTrafficSim/Blueprint/SimpleTrafficSim/Blueprints/RoadSpline/BP_SplineLane.BP_SplineLane_C|GetSpline _array_element) _index (+ (* (* (Variables|Input|GetLaneWdith) _array_index) (Math|Vector|GetRightVector (Spline|GetRotationatSplinePoint _spline_2 _index "World"))) (+ (Spline|GetLocationatSplinePoint _spline_2 _index "World") (* (Math|Vector|GetRightVector (Spline|GetRotationatSplinePoint _spline_2 _index "World")) -1.0 (* (Variables|Input|GetLaneWdith) (- (Math|Conversions|ToFloat(Integer) (/ (Variables|Input|GetlaneNumIn) 2)) 0.5))))) "World" true)
              (Spline|SetRotationatSplinePoint (Variables|/SimpleTrafficSim/Blueprint/SimpleTrafficSim/Blueprints/RoadSpline/BP_SplineLane.BP_SplineLane_C|GetSpline _array_element) _index (Spline|GetRotationatSplinePoint _spline_2 _index "World") "World" true)
              (Spline|SetTangentatSplinePoint (Variables|/SimpleTrafficSim/Blueprint/SimpleTrafficSim/Blueprints/RoadSpline/BP_SplineLane.BP_SplineLane_C|GetSpline _array_element) _index (Spline|GetTangentatSplinePoint (Variables|Default|GetSpline) _index "World") "World" true))))
        (for _index_2 (range (Spline|GetNumberOfSplinePoints (Variables|Default|GetSpline)) (LocalVariables|GetCurSplinePointNum))
          (Spline|RemoveSplinePoint (Variables|/SimpleTrafficSim/Blueprint/SimpleTrafficSim/Blueprints/RoadSpline/BP_SplineLane.BP_SplineLane_C|GetSpline _array_element) _index_2 true))
        ;[1 1 1] Set BillBoard
        (Utilities|IsValid (Variables|/SimpleTrafficSim/Blueprint/SimpleTrafficSim/Blueprints/RoadSpline/BP_SplineLane.BP_SplineLane_C|GetBillboard_start _array_element)
          (:Is%20Valid
            (Transformation|SetWorldLocation (Variables|/SimpleTrafficSim/Blueprint/SimpleTrafficSim/Blueprints/RoadSpline/BP_SplineLane.BP_SplineLane_C|GetBillboard_start _array_element) (+ (Spline|GetLocationatSplinePoint (Variables|/SimpleTrafficSim/Blueprint/SimpleTrafficSim/Blueprints/RoadSpline/BP_SplineLane.BP_SplineLane_C|GetSpline _array_element) 0 "World") (LocalVariables|GetSpriteOffset)) false false)
            (Transformation|SetWorldLocation (Variables|/SimpleTrafficSim/Blueprint/SimpleTrafficSim/Blueprints/RoadSpline/BP_SplineLane.BP_SplineLane_C|GetBillboard_end _array_element) (+ (Spline|GetLocationatSplinePoint (Variables|/SimpleTrafficSim/Blueprint/SimpleTrafficSim/Blueprints/RoadSpline/BP_SplineLane.BP_SplineLane_C|GetSpline _array_element) (Class|SplineComponent|GetNumberOfSplineSegments (Variables|/SimpleTrafficSim/Blueprint/SimpleTrafficSim/Blueprints/RoadSpline/BP_SplineLane.BP_SplineLane_C|GetSpline _array_element)) "World") (LocalVariables|GetSpriteOffset)) false false))))
      (:Is%20Not%20Valid
        (Class|DimensioBPLibrary|PrintLog (Utilities|String|Append "Faild to Construct:" (Utilities|GetDisplayName self) " Lane is Invalid index:" (Utilities|String|ToString(Integer) _array_index) " in " (Utilities|String|ToString(Integer) (Utilities|Array|Length _lanes))))))))

(fn SetSplinePoint
  (params (Spline :type Spline%20Component%20Object%20Reference) (Index :type Integer)))

(fn PickMeshPosition
  (bind _offset (LocalVariables|GetOffset))
  (bind _spline (Variables|Default|GetSpline))
  (bind _tagscale (Variables|Default|GetTagScale))
  (bind _returnvalue (Spline|GetNumberOfSplinePoints _spline))
  (bind _returnvalue_2 (Spline|GetTransformatSplinePoint _spline 0 "World" false))
  (bind _returnvalue_3 (Math|Conversions|ToVector(Float) _tagscale))
  (bind (_location _rotation) (Math|Transform|BreakTransform _returnvalue_2))
  (bind _returnvalue_4 (- _returnvalue 1))
  (bind _returnvalue_5 (Spline|GetTransformatSplinePoint _spline _returnvalue_4 "World" false))
  (bind (_location_2 _rotation_2) (Math|Transform|BreakTransform _returnvalue_5))
  (Utilities|FlowControl|Sequence
    (:then_0
      (Transformation|SetWorldTransform (Variables|Default|GetBillboard_Start) (Math|Transform|MakeTransform (+ _location _offset) _rotation _returnvalue_3) false false))
    (:then_1
      (Transformation|SetWorldTransform (Variables|Default|GetBillboard_End) (Math|Transform|MakeTransform (+ _location_2 _offset) _rotation_2 _returnvalue_3) false false))))

(fn ConstructFunc
  (CallFunction|LanePosition)
  (CallFunction|PickMeshPosition))

(fn GetAttachedLanes
  (bind _outactors (Actor|GetAttachedActors true true))
  (bind _self self)
  (bind _returnvalue (Utilities|GetDisplayName _self))
  (Utilities|Array|Clear (Variables|Road|GetLanes))
  (Class|DimensioBPLibrary|PrintLog (Utilities|String|Append "attachend Num:" (Utilities|String|ToString(Integer) (Utilities|Array|Length _outactors))))
  (for _array_element _outactors
    (bind _asbp_spline_lane (Utilities|Casting|CastToBP_SplineLane _array_element)
      (:then
        (Utilities|Array|Add (Variables|Road|GetLanes) _asbp_spline_lane)
        (Class|DimensioBPLibrary|PrintLog (Utilities|String|Append (Utilities|GetDisplayName _array_element) "Attached to :" _returnvalue)))
      (:CastFailed
        (Class|DimensioBPLibrary|PrintLog (Utilities|String|Append (Utilities|GetDisplayName _array_element) "is Non-SplineLane Actor attached to" _returnvalue))))))

(fn SpawnLanesbyNum
  (params (LaneNum :type Integer))
  (Utilities|FlowControl|Sequence
    (:then_0
      (for _array_element (Variables|Road|GetLanes)
        (Actor|DestroyActor _array_element))
      (Utilities|Array|Clear (Variables|Road|GetLanes)))
    (:then_1
      (for _index (range 1 LaneNum)
        (bind _returnvalue (Game|SpawnActorfromClass "/SimpleTrafficSim/Blueprint/SimpleTrafficSim/Blueprints/RoadSpline/BP_SplineLane.BP_SplineLane_C" (Transformation|GetActorTransform) "Undefined" 0 0))
        (Utilities|Array|Add (Variables|Road|GetLanes) _returnvalue)
        (Transformation|AttachActorToActor _returnvalue self "Lanes" "KeepRelative" "KeepRelative" "KeepRelative" true)))))

(fn NewFunction)

(fn TraceHeight
  (params (Height :type Float%20%28double-precision%29))
  (bind _spline (Variables|Default|GetSpline))
  (bind _returnvalue (Class|SplineComponent|GetUpVectoratSplinePoint _spline 0 "World"))
  (bind _returnvalue_2 (* _returnvalue 5e+02))
  (for _index (range 0 (- (Spline|GetNumberOfSplinePoints (Variables|Default|GetSpline)) 1))
    (bind _outhit (Collision|LineTraceByChannel (+ (Spline|GetLocationatSplinePoint _spline _index "World") _returnvalue_2) (+ (Spline|GetLocationatSplinePoint _spline _index "World") (* _returnvalue_2 -1.0)) "TraceTypeQuery1" true 0 "ForDuration" true "(R=1.000000,G=0.000000,B=0.000000,A=1.000000)" "(R=0.000000,G=1.000000,B=0.000000,A=1.000000)" 3.0))
    (if (.bBlockingHit (Collision|BreakHitResult _outhit))
      (Spline|SetLocationatSplinePoint (Variables|Default|GetSpline) _index (+ (.Location (Collision|BreakHitResult _outhit)) (+ (.Normal (Collision|BreakHitResult _outhit)) Height)) "World" true)
      (else
        (Class|DimensioBPLibrary|PrintLog (Utilities|String|Append (Utilities|GetObjectName self) " miss tracing at: " (Utilities|String|ToString(Integer) _index)) true true "(R=0.000000,G=0.660000,B=1.000000,A=1.000000)" 2.0 "Warning")))))

(fn CopySpline
  (params (InvertNewTrans :type Transform))
  (bind _spline (Variables|Default|GetSpline))
  (bind _spline_2 (Variables|Default|GetSpline))
  (bind _returnvalue (Spline|GetNumberOfSplinePoints _spline_2))
  (bind _returnvalue_2 (- _returnvalue 1))
  (for _index (range 0 _returnvalue_2)
    (Utilities|Array|Add (LocalVariables|GetSplinePoints) (Utilities|Struct|MakeSplinePoint (Math|Conversions|ToFloat(Integer) (- _returnvalue_2 _index)) (Math|Vector|SelectVector (+ (Math|Transform|TransformLocation InvertNewTrans (Spline|GetLocationatSplinePoint _spline _index "World")) (* (Math|Vector|Normalize (Math|Transform|TransformDirection InvertNewTrans (* (Spline|GetArriveTangentatSplinePoint _spline _index "World") -1.0))) 2e+02)) (Math|Transform|TransformLocation InvertNewTrans (Spline|GetLocationatSplinePoint _spline _index "World")) (or (== _index 0) (== _index _returnvalue_2))) (Math|Transform|TransformDirection InvertNewTrans (* (Spline|GetArriveTangentatSplinePoint _spline _index "World") -1.0)) (Math|Transform|TransformDirection InvertNewTrans (* (Spline|GetLeaveTangentatSplinePoint _spline _index "World") -1.0)) (Spline|GetRotationatSplinePoint _spline _index "Local") "1.000000,1.000000,1.000000" (Class|SplineComponent|GetSplinePointType (Variables|Default|GetSpline) _index))))
  (return (LocalVariables|GetSplinePoints)))

(fn ApplySpline
  (params (NewSpline :type Array%20of%20Spline%20Point%20Structures))
  (bind _spline (Variables|Default|GetSpline))
  (LocalVariables|SetReverse NewSpline)
  (Spline|ClearSplinePoints _spline true)
  (Class|SplineComponent|AddPoints _spline (LocalVariables|GetReverse) true)
  (CallFunction|ConstructFunc))

(fn GetSwichabledLane
  (params (CurLane :type BP%20Spline%20Lane%20Object%20Reference))
  (return (Helper|GetNeibourLane (Utilities|Array|FindItem (Variables|Road|GetLanes) CurLane))))

(fn GetNeibourLane
  (params (Idx :type Integer))
  (bind _returnvalue (+ Idx 1))
  (bind _returnvalue_2 (- Idx 1))
  (Utilities|FlowControl|Sequence
    (:then_0
      (if (< _returnvalue (Utilities|Array|Length (Variables|Road|GetLanes)))
        (Utilities|Array|Add (LocalVariables|GetLanes) (Utilities|Array|Get(acopy) (Variables|Road|GetLanes) _returnvalue))))
    (:then_1
      (if (>= _returnvalue_2 0)
        (Utilities|Array|Add (LocalVariables|GetLanes) (Utilities|Array|Get(acopy) (Variables|Road|GetLanes) _returnvalue_2))))
    (:then_2
      (return (LocalVariables|GetLanes)))))