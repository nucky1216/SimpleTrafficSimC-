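; Debug actor in the traffic sim's road spline folder that live-tunes four parameters on a referenced CarCube: frequency, Z drag, R delay and Frac.
; Each Tick compares the input values against cached copies.
; When any differs, it refreshes the cache and pushes all four inputs to CarCube, so edits take effect while running.
; BeginPlay, overlap and the construction script are empty.
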(event EventBeginPlay)

(event Collision|EventActorBeginOverlap
  (params (OtherActor :type Actor%20Object%20Reference)))

(event EventTick
  (params (DeltaSeconds :type Float%20%28single-precision%29))
  (bind _carcube (Variables|Default|GetCarCube))
  (if (Math|Boolean|ORBoolean (!= (Variables|Default|GetIn%20Freq) (Variables|Default|GetFreq)) (!= (Variables|Default|GetIn%20ZDrag) (Variables|Default|GetZDrag)) (!= (Variables|Default|GetIn%20RDelay) (Variables|Default|GetRDelay)) (!= (Variables|Default|GetFrac) (Variables|Default|GetIn%20Frac)))
    (Variables|Default|SetFreq (Variables|Default|GetIn%20Freq))
    (Variables|Default|SetZDrag (Variables|Default|GetIn%20ZDrag))
    (Variables|Default|SetRDelay (Variables|Default|GetIn%20RDelay))
    (Variables|Default|SetFrac (Variables|Default|GetIn%20Frac))
    (Variables|/SimpleTrafficSim/Blueprint/SimpleTrafficSim/Blueprints/BP_CarCube.BP_CarCube_C|SetIn%20Frac _carcube (Variables|Default|GetIn%20Frac))
    (Variables|/SimpleTrafficSim/Blueprint/SimpleTrafficSim/Blueprints/BP_CarCube.BP_CarCube_C|SetIn%20Freq _carcube (Variables|Default|GetIn%20Freq))
    (Variables|/SimpleTrafficSim/Blueprint/SimpleTrafficSim/Blueprints/BP_CarCube.BP_CarCube_C|SetIn%20ZDrag _carcube (Variables|Default|GetIn%20ZDrag))
    (Variables|/SimpleTrafficSim/Blueprint/SimpleTrafficSim/Blueprints/BP_CarCube.BP_CarCube_C|SetIn%20RDelay _carcube (Variables|Default|GetIn%20RDelay))))

(fn ConstructionScript)