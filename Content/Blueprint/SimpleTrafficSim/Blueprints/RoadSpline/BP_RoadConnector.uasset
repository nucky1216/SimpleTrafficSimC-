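; Road connector for the traffic sim that joins road lanes and, at crossroads, runs traffic lights.
; Construction rebuilds connector splines from auto-paired segments and manual lane links, plus trigger boxes at lane ends and editor billboards.
; Overlapping cars get a random next spline and halt on non-green, with the first held car released on green.
; A looping timer restarts a Delay-chained cycle over two light groups, each with straight/right and optional left phases.
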(event Custom|LightChange
  (bind _unifiedtime (Variables|LightTime|GetUnifiedTime))
  (bind _leftgreen_2_time (Variables|Lights2|GetLeftGreen%202%20Time))
  (bind _leftgreentime (Variables|LightTime|GetLeftGreenTime))
  (bind _unifiedtime_2 (Variables|LightTime|GetUnifiedTime))
  (bind _left_green_1_time (Variables|Lights1|GetLeft%20Green%201%20Time))
  (bind _leftgreentime_2 (Variables|LightTime|GetLeftGreenTime))
  (bind _returnvalue (Math|Float|SelectFloat _leftgreentime _leftgreen_2_time _unifiedtime))
  (bind _returnvalue_2 (Math|Float|SelectFloat _leftgreentime_2 _left_green_1_time _unifiedtime_2))
  ;[0.1273 1 0.1149] Light1 StraightRight Green
  (SignalLight|SignalLightState "NewEnumerator2" "NewEnumerator0")
  (SignalLight|SignalLightState "NewEnumerator2" "NewEnumerator2")
  (Utilities|FlowControl|Delay (Math|Float|SelectFloat (Variables|LightTime|GetGreenTime) (Variables|Lights1|GetGreen%201%20Time) (Variables|LightTime|GetUnifiedTime)))
  ;[1 0.908 0.1237] Light1 StraightRight Yellow
  (SignalLight|SignalLightState "NewEnumerator1" "NewEnumerator0")
  (SignalLight|SignalLightState "NewEnumerator1" "NewEnumerator2")
  (Utilities|FlowControl|Delay (Math|Float|SelectFloat (Variables|LightTime|GetYellowTime) (Variables|Lights1|GetYellow%201%20Time) (Variables|LightTime|GetUnifiedTime)))
  ;[1 0.09722 0.01955] Light1 Red
  (SignalLight|SignalLightState "NewEnumerator0" "NewEnumerator6")
  ;[1 0.1838 0.8072] Wait for the Running Car Pass
  (Utilities|FlowControl|Delay (Variables|LightTime|GetSwitchDelay))
  (if (!= _returnvalue_2 0.0)
    ;[0.2148 1 0.09434] Light1 Left Green
    (SignalLight|SignalLightState "NewEnumerator2" "NewEnumerator4")
    (Utilities|FlowControl|Delay _returnvalue_2)
    ;[1 0.8266 0.02494] Light 1 Left Yellow
    (SignalLight|SignalLightState "NewEnumerator1" "NewEnumerator4")
    (Utilities|FlowControl|Delay (Math|Float|SelectFloat (Variables|LightTime|GetYellowTime) (Variables|Lights1|GetYellow%201%20Time) (Variables|LightTime|GetUnifiedTime)))
    (SignalLight|SignalLightState "NewEnumerator0" "NewEnumerator4"))
  (Utilities|FlowControl|Delay (Variables|LightTime|GetSwitchDelay))
  ;[0.1273 1 0.1149] Light2 StraightRight Green
  (SignalLight|SignalLightState "NewEnumerator2" "NewEnumerator1")
  (SignalLight|SignalLightState "NewEnumerator2" "NewEnumerator3")
  (Utilities|FlowControl|Delay (Math|Float|SelectFloat (Variables|LightTime|GetGreenTime) (Variables|Lights2|GetGreen%202%20Time) (Variables|LightTime|GetUnifiedTime)))
  ;[1 0.908 0.1237] Light2 StraightRight Yellow
  (SignalLight|SignalLightState "NewEnumerator1" "NewEnumerator1")
  (SignalLight|SignalLightState "NewEnumerator1" "NewEnumerator3")
  (Utilities|FlowControl|Delay (Math|Float|SelectFloat (Variables|LightTime|GetYellowTime) (Variables|Lights2|GetYellow%202%20Time) (Variables|LightTime|GetUnifiedTime)))
  ;[1 0.09722 0.01955] Light2 Red
  (SignalLight|SignalLightState "NewEnumerator0" "NewEnumerator7")
  ;[1 0.1838 0.8072] Wait for the Running Car Pass
  (Utilities|FlowControl|Delay (Variables|LightTime|GetSwitchDelay))
  (if (!= _returnvalue 0.0)
    ;[0.2148 1 0.09434] Light2 Left Green
    (SignalLight|SignalLightState "NewEnumerator2" "NewEnumerator5")
    (Utilities|FlowControl|Delay _returnvalue)
    ;[1 0.8266 0.02494] Light2 Left Yellow
    (SignalLight|SignalLightState "NewEnumerator1" "NewEnumerator5")
    (Utilities|FlowControl|Delay (Math|Float|SelectFloat (Variables|LightTime|GetYellowTime) (Variables|Lights2|GetYellow%202%20Time) (Variables|LightTime|GetUnifiedTime)))
    (SignalLight|SignalLightState "NewEnumerator0" "NewEnumerator5")))

(event Custom|ShowBox
  (Debug|DebugDrawBox))

(event EventBeginPlay
  (bind _unifiedtime (Variables|LightTime|GetUnifiedTime))
  (bind _leftgreen_2_time (Variables|Lights2|GetLeftGreen%202%20Time))
  (bind _leftgreentime (Variables|LightTime|GetLeftGreenTime))
  (bind _unifiedtime_2 (Variables|LightTime|GetUnifiedTime))
  (bind _left_green_1_time (Variables|Lights1|GetLeft%20Green%201%20Time))
  (bind _leftgreentime_2 (Variables|LightTime|GetLeftGreenTime))
  (bind _returnvalue (Math|Float|SelectFloat _leftgreentime _leftgreen_2_time _unifiedtime))
  (bind _returnvalue_2 (Math|Float|SelectFloat _leftgreentime_2 _left_green_1_time _unifiedtime_2))
  (|CallParentFunction)
  (Utilities|FlowControl|Sequence
    (:then_0
      (if (not (Variables|Connector|GetNot%20Cross%20Road))
        (Utilities|Time|SetTimerbyEvent (delegate Custom|LightChange) (Math|Float|SelectFloat (+ (* (Variables|LightTime|GetGreenTime) 2.0) (* (Variables|LightTime|GetYellowTime) (Math|Float|SelectFloat 2.0 4.0 (== (Variables|LightTime|GetLeftGreenTime) 0.0))) (* (Variables|LightTime|GetLeftGreenTime) 2.0) (* (Variables|LightTime|GetSwitchDelay) 2.0)) (+ (Variables|Lights1|GetGreen%201%20Time) (* (Variables|Lights1|GetYellow%201%20Time) (Math|Float|SelectFloat 1.0 2.0 (== (Variables|Lights1|GetLeft%20Green%201%20Time) 0.0))) (Variables|Lights1|GetLeft%20Green%201%20Time) (Variables|Lights2|GetGreen%202%20Time) (* (Variables|Lights2|GetYellow%202%20Time) (Math|Float|SelectFloat 1.0 2.0 (== (Variables|Lights2|GetLeftGreen%202%20Time) 0.0))) (Variables|Lights2|GetLeftGreen%202%20Time)) (Variables|LightTime|GetUnifiedTime)) true)))
    (:then_2
      (if (not (Variables|Connector|GetNot%20Cross%20Road))
        ;[0.1273 1 0.1149] Light1 StraightRight Green
        (SignalLight|SignalLightState "NewEnumerator2" "NewEnumerator0")
        (SignalLight|SignalLightState "NewEnumerator2" "NewEnumerator2")
        (Utilities|FlowControl|Delay (Math|Float|SelectFloat (Variables|LightTime|GetGreenTime) (Variables|Lights1|GetGreen%201%20Time) (Variables|LightTime|GetUnifiedTime)))
        ;[1 0.908 0.1237] Light1 StraightRight Yellow
        (SignalLight|SignalLightState "NewEnumerator1" "NewEnumerator0")
        (SignalLight|SignalLightState "NewEnumerator1" "NewEnumerator2")
        (Utilities|FlowControl|Delay (Math|Float|SelectFloat (Variables|LightTime|GetYellowTime) (Variables|Lights1|GetYellow%201%20Time) (Variables|LightTime|GetUnifiedTime)))
        ;[1 0.09722 0.01955] Light1 Red
        (SignalLight|SignalLightState "NewEnumerator0" "NewEnumerator6")
        ;[1 0.1838 0.8072] Wait for the Running Car Pass
        (Utilities|FlowControl|Delay (Variables|LightTime|GetSwitchDelay))
        (if (!= _returnvalue_2 0.0)
          ;[0.2148 1 0.09434] Light1 Left Green
          (SignalLight|SignalLightState "NewEnumerator2" "NewEnumerator4")
          (Utilities|FlowControl|Delay _returnvalue_2)
          ;[1 0.8266 0.02494] Light 1 Left Yellow
          (SignalLight|SignalLightState "NewEnumerator1" "NewEnumerator4")
          (Utilities|FlowControl|Delay (Math|Float|SelectFloat (Variables|LightTime|GetYellowTime) (Variables|Lights1|GetYellow%201%20Time) (Variables|LightTime|GetUnifiedTime)))
          (SignalLight|SignalLightState "NewEnumerator0" "NewEnumerator4"))
        (Utilities|FlowControl|Delay (Variables|LightTime|GetSwitchDelay))
        ;[0.1273 1 0.1149] Light2 StraightRight Green
        (SignalLight|SignalLightState "NewEnumerator2" "NewEnumerator1")
        (SignalLight|SignalLightState "NewEnumerator2" "NewEnumerator3")
        (Utilities|FlowControl|Delay (Math|Float|SelectFloat (Variables|LightTime|GetGreenTime) (Variables|Lights2|GetGreen%202%20Time) (Variables|LightTime|GetUnifiedTime)))
        ;[1 0.908 0.1237] Light2 StraightRight Yellow
        (SignalLight|SignalLightState "NewEnumerator1" "NewEnumerator1")
        (SignalLight|SignalLightState "NewEnumerator1" "NewEnumerator3")
        (Utilities|FlowControl|Delay (Math|Float|SelectFloat (Variables|LightTime|GetYellowTime) (Variables|Lights2|GetYellow%202%20Time) (Variables|LightTime|GetUnifiedTime)))
        ;[1 0.09722 0.01955] Light2 Red
        (SignalLight|SignalLightState "NewEnumerator0" "NewEnumerator7")
        ;[1 0.1838 0.8072] Wait for the Running Car Pass
        (Utilities|FlowControl|Delay (Variables|LightTime|GetSwitchDelay))
        (if (!= _returnvalue 0.0)
          ;[0.2148 1 0.09434] Light2 Left Green
          (SignalLight|SignalLightState "NewEnumerator2" "NewEnumerator5")
          (Utilities|FlowControl|Delay _returnvalue)
          ;[1 0.8266 0.02494] Light2 Left Yellow
          (SignalLight|SignalLightState "NewEnumerator1" "NewEnumerator5")
          (Utilities|FlowControl|Delay (Math|Float|SelectFloat (Variables|LightTime|GetYellowTime) (Variables|Lights2|GetYellow%202%20Time) (Variables|LightTime|GetUnifiedTime)))
          (SignalLight|SignalLightState "NewEnumerator0" "NewEnumerator5"))))))

(event EventTick
  (params (DeltaSeconds :type Float%20%28single-precision%29)))

(fn ConstructionScript
  (|CallParentFunction)
  (CallFunction|ConstructFunc))

(fn AutoConnect
  (params (FullConnect :type Boolean) (MatchedOrder :type Boolean) (ExcludeLeft :type Boolean))
  (bind _segpairs (Variables|Connector|GetSegPairs))
  (bind _keys (Utilities|Map|Keys _segpairs))
  (for _array_element _keys
    (Utilities|Array|Clear (LocalVariables|GetStrLanes))
    (Utilities|FlowControl|Sequence
      (:then_0
        (if ExcludeLeft
          (for _array_element_2 (Variables|/SimpleTrafficSim/Blueprint/SimpleTrafficSim/Blueprints/RoadSpline/BP_RoadSegment.BP_RoadSegment_C|GetLanes _array_element)
            (if (Utilities|Enum|Equal(Enum) (Variables|/SimpleTrafficSim/Blueprint/SimpleTrafficSim/Blueprints/RoadSpline/BP_SplineLane.BP_SplineLane_C|GetRoadType _array_element_2) "NewEnumerator0")
              (Utilities|Array|Add (LocalVariables|GetStrLanes) _array_element_2)))
          (else
            (LocalVariables|SetStrLanes (Variables|/SimpleTrafficSim/Blueprint/SimpleTrafficSim/Blueprints/RoadSpline/BP_RoadSegment.BP_RoadSegment_C|GetLanes _array_element)))))
      (:then_1
        (LocalVariables|SetEndLanes (Variables|/SimpleTrafficSim/Blueprint/SimpleTrafficSim/Blueprints/RoadSpline/BP_RoadSegment.BP_RoadSegment_C|GetLanes (.Value (Utilities|Map|Find _segpairs _array_element))))
        (if (not MatchedOrder)
          (Utilities|Array|Reverse (LocalVariables|GetStrLanes))
          (Utilities|Array|Reverse (LocalVariables|GetEndLanes))))
      (:then_2
        (for (_array_element_3 _array_index) (LocalVariables|GetStrLanes)
          (for (_array_element_4 _array_index_2) (LocalVariables|GetEndLanes)
            (if FullConnect
              (Connector|ConnectALane _array_element_3 _array_element_4 1.0 :!label _label)
              (elif (== _array_index_2 _array_index)
                (goto _label)))))))))

(fn ConnectALane
  (params (StartLane :type BP%20Spline%20Lane%20Object%20Reference) (EndLane :type BP%20Spline%20Lane%20Object%20Reference) (Curve :type Float%20%28double-precision%29))
  (bind _spline (Variables|/SimpleTrafficSim/Blueprint/SimpleTrafficSim/Blueprints/RoadSpline/BP_SplineLane.BP_SplineLane_C|GetSpline EndLane))
  (bind _starter_2_enders (Variables|Default|GetStarter%202%20Enders))
  (bind _spline_2 (Variables|/SimpleTrafficSim/Blueprint/SimpleTrafficSim/Blueprints/RoadSpline/BP_SplineLane.BP_SplineLane_C|GetSpline StartLane))
  (bind _boxscale (Variables|Default|GetBoxScale))
  (bind _returnvalue (Spline|GetNumberOfSplinePoints _spline_2))
  (bind _value (Utilities|Map|Find _starter_2_enders StartLane))
  (bind (_enders _splines) (Utilities|Struct|BreakS_EndersSplines _value))
  (bind _returnvalue_2 (- _returnvalue 1))
  (bind _returnvalue_3 (Spline|GetTangentatSplinePoint _spline_2 _returnvalue_2 "World"))
  (bind _returnvalue_4 (Spline|GetLocationatSplinePoint _spline_2 _returnvalue_2 "World"))
  (bind _returnvalue_5 (Math|Conversions|RotationFromXVector _returnvalue_3))
  (Utilities|IsValid StartLane
    (:Is%20Valid
      (Utilities|FlowControl|Sequence
        (:then_0
          (Debug|SpawnCollosionBox (Math|Transform|MakeTransform (+ (* (Math|Vector|GetForwardVector _returnvalue_5) (* (.X (Class|KismetMathLibrary|BreakVector3f _boxscale)) 1e+02)) _returnvalue_4 "0.000000,0.000000,100.000000") _returnvalue_5 _boxscale) StartLane)
          (bind _returnvalue_6 (AddComponent|AddSplineComponent true))
          (Variables|/Script/Engine.ActorComponent|SetComponentTags _returnvalue_6 (Utilities|Array|MakeArray "Connector"))
          (Spline|SetSplinePoints _returnvalue_6 (Utilities|Array|MakeArray _returnvalue_4 (Spline|GetLocationatSplinePoint _spline 0 "World")) "World" true)
          (Spline|SetTangentatSplinePoint _returnvalue_6 0 (* _returnvalue_3 Curve) "World" true)
          (Spline|SetTangentatSplinePoint _returnvalue_6 1 (* Curve (Spline|GetTangentatSplinePoint _spline 0 "World")) "World" true)
          (Utilities|Array|AddUnique (Variables|Default|GetSplineComponents) _returnvalue_6)
          ;[1 1 1] Insert the Struct Array Into  Map
          (bind _output_get (LocalVariables|SetEnders _enders))
          (Utilities|Array|AddUnique _output_get EndLane)
          (bind _output_get_2 (LocalVariables|SetSplines _splines))
          (Utilities|Array|AddUnique _output_get_2 _returnvalue_6)
          (Utilities|Map|Add _starter_2_enders StartLane (Utilities|Struct|MakeS_EndersSplines (LocalVariables|GetEnders) (LocalVariables|GetSplines))))))))

(fn ManualConnect
  (bind _lane_2_lanes (Variables|Connector|GetLane%202%20Lanes))
  (bind _keys (Utilities|Map|Keys _lane_2_lanes))
  (for _array_element _keys
    (for _array_element_2 (.Drivers (Utilities|Struct|BreakS_DrivePaths (.Value (Utilities|Map|Find _lane_2_lanes _array_element))))
      (if (not (Utilities|Array|ContainsItem (.Enders (Utilities|Struct|BreakS_EndersSplines (.Value (Utilities|Map|Find (Variables|Default|GetStarter%202%20Enders) _array_element)))) _array_element_2))
        (Connector|ConnectALane _array_element _array_element_2 (.Curve (Utilities|Struct|BreakS_DrivePaths (.Value (Utilities|Map|Find _lane_2_lanes _array_element)))))))))

(fn DebugDrawBox
  (for _array_element (Variables|Default|GetAllColBoxes)
    (Rendering|Debug|DrawDebugBox :Center (Transformation|GetWorldLocation _array_element) :Extent (Components|Box|GetScaledBoxExtent _array_element) :Rotation (Transformation|GetWorldRotation _array_element) :Duration 5.0 :Thickness 1e+01)))

(fn SpawnCollosionBox
  (params (RelativeTransform :type Transform) (StartLane :type BP%20Spline%20Lane%20Object%20Reference))
  (bind _roadtype (Variables|/SimpleTrafficSim/Blueprint/SimpleTrafficSim/Blueprints/RoadSpline/BP_SplineLane.BP_SplineLane_C|GetRoadType StartLane))
  (if (not (.ReturnValue (Utilities|Map|Find (Variables|Default|GetStarter%202%20Enders) StartLane)))
    (bind _returnvalue (AddComponent|AddBoxComponent true RelativeTransform))
    (LocalVariables|SetColBox _returnvalue)
    (Collision|BindEventtoOnComponentBeginOverlap _returnvalue (EventDispatchers|CreateEvent :!event OverlapACar))
    (Utilities|Array|AddUnique (Variables|Default|GetAllColBoxes) (LocalVariables|GetColBox))
    (Utilities|Map|Add (Variables|Default|GetBox%202%20Starter) _returnvalue StartLane)
    (Utilities|Map|Add (Variables|Default|GetBox%202%20Lights) _returnvalue "NewEnumerator2")
    (switch Utilities|FlowControl|Switch|SwitchonE_CrossLightGroup (Variables|/SimpleTrafficSim/Blueprint/SimpleTrafficSim/Blueprints/RoadSpline/BP_SplineLane.BP_SplineLane_C|GetLightGroup StartLane)
      (:NewEnumerator0
        (Utilities|Array|Add (Utilities|Select :Index _roadtype :NewEnumerator0 (Variables|Lights1|GetStraight1) :NewEnumerator1 (Variables|Lights1|GetLeft1) :NewEnumerator2 (Variables|Lights1|GetRight1)) (LocalVariables|GetColBox))
        (Utilities|Array|Add (Variables|Lights1|GetLightsGroup1) (LocalVariables|GetColBox)))
      (:NewEnumerator1
        (Utilities|Array|Add (Utilities|Select :Index _roadtype :NewEnumerator0 (Variables|Lights2|GetStraight2) :NewEnumerator1 (Variables|Lights2|GetLeft2) :NewEnumerator2 (Variables|Lights2|GetLeft2)) (LocalVariables|GetColBox))
        (Utilities|Array|Add (Variables|Lights2|GetLightsGroup2) (LocalVariables|GetColBox))))
    (Variables|/Script/Engine.ActorComponent|SetComponentTags (LocalVariables|GetColBox) (Utilities|Array|MakeArray (Utilities|String|StringToName (Variables|/SimpleTrafficSim/Blueprint/SimpleTrafficSim/Blueprints/RoadSpline/BP_SplineLane.BP_SplineLane_C|GetSegID StartLane))))))

(fn ClearVars
  (bind _splinecomponents (Variables|Default|GetSplineComponents))
  (bind _groupbillboards (Variables|Default|GetGroupBillBoards))
  (Utilities|FlowControl|Sequence
    (:then_0
      (Utilities|Map|Clear (Variables|Default|GetBox%202%20Starter))
      (Utilities|Map|Clear (Variables|Default|GetStarter%202%20Enders)))
    (:then_1
      (for _array_element (Variables|Default|GetAllColBoxes)
        (Components|DestroyComponent _array_element))
      (Utilities|Array|Clear (Variables|Default|GetAllColBoxes)))
    (:then_2
      (Utilities|Array|Clear (Variables|Lights1|GetStraight1))
      (Utilities|Array|Clear (Variables|Lights1|GetRight1))
      (Utilities|Array|Clear (Variables|Lights1|GetLeft1))
      (Utilities|Array|Clear (Variables|Lights2|GetStraight2))
      (Utilities|Array|Clear (Variables|Lights2|GetRight2))
      (Utilities|Array|Clear (Variables|Lights2|GetLeft2))
      (Utilities|Array|Clear (Variables|Lights1|GetLightsGroup1))
      (Utilities|Array|Clear (Variables|Lights2|GetLightsGroup2))
      (Utilities|Map|Clear (Variables|Default|GetBox%202%20Lights)))
    (:then_3
      (for _array_element_2 _splinecomponents
        (Utilities|IsValid _array_element_2
          (:Is%20Valid
            (Components|DestroyComponent _array_element_2))))
      (Utilities|Array|Clear _splinecomponents))
    (:then_4
      (for _array_element_3 _groupbillboards
        (Utilities|IsValid _array_element_3
          (:Is%20Valid
            (Components|DestroyComponent _array_element_3))))
      (Utilities|Array|Clear _groupbillboards))
    (:then_5
      (Utilities|Array|Clear (Variables|Default|GetTLSPosition)))))

(fn ChooseSpline
  (params (Box :type Box%20Component%20Object%20Reference))
  (bind _box_2_starter (Variables|Default|GetBox%202%20Starter))
  (bind _starter_2_enders (Variables|Default|GetStarter%202%20Enders))
  (bind _value (Utilities|Map|Find _box_2_starter Box))
  (bind _value_2 (Utilities|Map|Find _starter_2_enders _value))
  (bind _splines (Utilities|Struct|BreakS_EndersSplines _value_2))
  (return (Utilities|Array|Get(acopy) _splines (Math|Random|RandomInteger (Utilities|Array|Length _splines))) true))

(fn OverlapACar
  (params (OverlappedComponent :type Primitive%20Component%20Object%20Reference) (OtherActor :type Actor%20Object%20Reference) (OtherComp :type Primitive%20Component%20Object%20Reference) (OtherBodyIndex :type Integer) (bFromSweep :type Boolean) (SweepResult :type Hit%20Result%20Structure%20%28by%20ref%29))
  (bind _returnvalue (Actor|GetComponentbyClass OtherActor "/SimpleTrafficSim/Blueprint/SimpleTrafficSim/Blueprints/BPC_SimMovement.BPC_SimMovement_C"))
  (bind _asbox_collision (Utilities|Casting|CastToBoxComponent OverlappedComponent))
  (bind _box_2_lights (Variables|Default|GetBox%202%20Lights))
  (bind _value (Utilities|Map|Find _box_2_lights _asbox_collision))
  (bind _returnvalue_2 (Utilities|Enum|Equal(Enum) _value "NewEnumerator2"))
  (Utilities|IsValid _returnvalue
    (:Is%20Valid
      (if (== (Variables|/SimpleTrafficSim/Blueprint/SimpleTrafficSim/Blueprints/RoadSpline/BP_SplineLane.BP_SplineLane_C|GetSpline (.Value (Utilities|Map|Find (Variables|Default|GetBox%202%20Starter) _asbox_collision))) (Variables|/SimpleTrafficSim/Blueprint/SimpleTrafficSim/Blueprints/BPC_SimMovement.BPC_SimMovement_C|GetSpline _returnvalue))
        (Variables|/SimpleTrafficSim/Blueprint/SimpleTrafficSim/Blueprints/BPC_SimMovement.BPC_SimMovement_C|SetNextSpline _returnvalue (.Spline (CarDrive|ChooseSpline _asbox_collision)))
        (Utilities|FlowControl|Sequence
          (:then_0
            (if (not _returnvalue_2)
              (Variables|/SimpleTrafficSim/Blueprint/SimpleTrafficSim/Blueprints/BPC_SimMovement.BPC_SimMovement_C|SetExpectSpeed _returnvalue 0.0)))
          (:then_1
            (if (and (not _returnvalue_2) (not (.ReturnValue (Utilities|Map|Find (Variables|Default|GetBox%202%20StoppedCar) _asbox_collision))))
              (Variables|/SimpleTrafficSim/Blueprint/SimpleTrafficSim/Blueprints/BPC_SimMovement.BPC_SimMovement_C|SetStoppedBySignal _returnvalue true)
              (Utilities|Map|Add (Variables|Default|GetBox%202%20StoppedCar) _asbox_collision _returnvalue))))))))

(fn SignalLightState
  (params (SetState :type E_LightState%20Enum :default "NewEnumerator0") (LightGroup :type E_LightsGroupType%20Enum :default "NewEnumerator0"))
  (bind _output_get (LocalVariables|SetColBoxArray (Utilities|FindBoxesbyLightGroup LightGroup)))
  (for _array_element _output_get
    (Utilities|Map|Add (Variables|Default|GetBox%202%20Lights) _array_element SetState)
    (Utilities|FlowControl|Sequence
      (:then_0
        (if (Utilities|Enum|Equal(Enum) SetState "NewEnumerator2")
          (if (.ReturnValue (Utilities|Map|Find (Variables|Default|GetBox%202%20StoppedCar) _array_element))
            (Utilities|IsValid (.Value (Utilities|Map|Find (Variables|Default|GetBox%202%20StoppedCar) _array_element))
              (:Is%20Valid
                (Variables|/SimpleTrafficSim/Blueprint/SimpleTrafficSim/Blueprints/BPC_SimMovement.BPC_SimMovement_C|SetExpectSpeed (.Value (Utilities|Map|Find (Variables|Default|GetBox%202%20StoppedCar) _array_element)) (Variables|/SimpleTrafficSim/Blueprint/SimpleTrafficSim/Blueprints/BPC_SimMovement.BPC_SimMovement_C|GetMaxSpeed (.Value (Utilities|Map|Find (Variables|Default|GetBox%202%20StoppedCar) _array_element))))
                (Variables|/SimpleTrafficSim/Blueprint/SimpleTrafficSim/Blueprints/BPC_SimMovement.BPC_SimMovement_C|SetStoppedBySignal (.Value (Utilities|Map|Find (Variables|Default|GetBox%202%20StoppedCar) _array_element)) false))
              (:Is%20Not%20Valid
                _))
            (Utilities|Map|Remove (Variables|Default|GetBox%202%20StoppedCar) _array_element))))))
  (Default|CallTSLChange SetState LightGroup))

(fn ConstructFunc
  (bind _not_cross_road (Variables|Connector|GetNot%20Cross%20Road))
  (bind _billboard (Variables|Default|GetBillboard))
  (CallFunction|ClearVars)
  (Connector|AutoConnect (Variables|Connector|GetFull%20Connect) (Variables|Connector|GetMatched%20Order) (Variables|Connector|GetExcludeLeft))
  (Connector|ManualConnect)
  (Rendering|Components|Sprite|SetSprite _billboard (select _not_cross_road "/SimpleTrafficSim/Blueprint/SimpleTrafficSim/Blueprints/DebugMaterial/T_Connect.T_Connect" "/SimpleTrafficSim/Blueprint/SimpleTrafficSim/Blueprints/DebugMaterial/T_TrafficLight.T_TrafficLight"))
  (Transformation|SetWorldScale3D _billboard (Math|Vector|SelectVector "2.000000,2.000000,2.000000" "5.000000,5.000000,5.000000" _not_cross_road))
  (CallFunction|SpawnGroupBiilboard))

(fn SpawnGroupBiilboard
  (Utilities|Array|AppendArray (Variables|Default|GetTLSPosition) (CallFunction|GetTSLPostion (Variables|Lights1|GetLightsGroup1)))
  (Utilities|Array|AppendArray (Variables|Default|GetTLSPosition) (CallFunction|GetTSLPostion (Variables|Lights2|GetLightsGroup2)))
  (for (_array_element _array_index) (Variables|Default|GetTLSPosition)
    (if (Utilities|Operators|NotEqual(!=) _array_element (Variables|Default|GetInvalidPosiiton) 0.0)
      (bind _returnvalue (AddComponent|AddBillboardComponent true (Math|Transform|MakeTransform (+ _array_element "0.000000,0.000000,200.000000") "0, 0, 0" "2.000000,2.000000,2.000000")))
      (Rendering|Components|Sprite|SetSprite _returnvalue (Utilities|Select :Index _array_index :Option%200 "/SimpleTrafficSim/Blueprint/SimpleTrafficSim/Blueprints/DebugMaterial/T_Number1.T_Number1" :Option%201 "/SimpleTrafficSim/Blueprint/SimpleTrafficSim/Blueprints/DebugMaterial/T_Number1.T_Number1" :Option%202 "/SimpleTrafficSim/Blueprint/SimpleTrafficSim/Blueprints/DebugMaterial/T_Number2.T_Number2" :Option%203 "/SimpleTrafficSim/Blueprint/SimpleTrafficSim/Blueprints/DebugMaterial/T_Number2.T_Number2"))
      (Utilities|Array|Add (Variables|Default|GetGroupBillBoards) _returnvalue))))

(fn GetTSLPostion
  (params (LightGroup :type Array%20of%20Box%20Component%20Object%20References))
  (bind _segids (LocalVariables|GetSegIDs))
  (bind _segids_2 (LocalVariables|GetSegIDs))
  (for _array_element LightGroup
    (if (.ReturnValue (Utilities|Map|Find (LocalVariables|GetSegIDs) (Utilities|Array|Get(acopy) (Variables|/Script/Engine.ActorComponent|GetComponentTags _array_element))))
      (Utilities|Map|Add _segids_2 (Utilities|Array|Get(acopy) (Variables|/Script/Engine.ActorComponent|GetComponentTags _array_element)) (+ (.Value (Utilities|Map|Find (LocalVariables|GetSegIDs) (Utilities|Array|Get(acopy) (Variables|/Script/Engine.ActorComponent|GetComponentTags _array_element)))) (Transformation|GetWorldLocation _array_element)))
      (else
        (Utilities|Map|Add _segids_2 (Utilities|Array|Get(acopy) (Variables|/Script/Engine.ActorComponent|GetComponentTags _array_element)) (Transformation|GetWorldLocation _array_element)))))
  (bind _keys (Utilities|Map|Keys _segids))
  (bind _values (Utilities|Map|Values _segids))
  (for _array_element_2 _values
    (Utilities|Array|Add (LocalVariables|GetPostions) (/ _array_element_2 (/ (Utilities|Array|Length LightGroup) (Utilities|Select :Index (Utilities|Array|Length _keys) :Option%200 1 :Option%201 1 :Option%202 2)))))
  (Utilities|FlowControl|Sequence
    (:then_0
      (if (< (Utilities|Array|Length _keys) 2)
        (Utilities|Array|Add (LocalVariables|GetPostions) (Variables|Default|GetInvalidPosiiton))))
    (:then_1
      (return (LocalVariables|GetPostions)))))