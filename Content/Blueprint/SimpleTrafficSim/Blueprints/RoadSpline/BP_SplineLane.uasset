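; BP_SplineLane is a road lane actor in the simple traffic simulation, built around a spline and a box.
; Construction offsets the box from the actor origin using its extent, and a debug helper can draw it.
; CheckLaneEmpty runs a straight, height-offset multi-object trace between two spline distances, returning false if a blocking hit's actor has a BPC_SimMovement component.
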(event EventBeginPlay)

(event Collision|EventActorBeginOverlap
  (params (OtherActor :type Actor%20Object%20Reference)))

(event EventTick
  (params (DeltaSeconds :type Float%20%28single-precision%29)))

(fn ConstructionScript
  (bind _box (Variables|Default|GetBox))
  (bind _returnvalue (Components|Box|GetScaledBoxExtent _box))
  (bind (_x _y _z) (Math|Vector|BreakVector _returnvalue))
  (Transformation|SetRelativeLocation _box (Math|Vector|MakeVector (* _x -1.0) 0.0 (/ _z 2.0)) false false))

(fn DrawBox
  (params (NewParam :type Float%20%28double-precision%29))
  (bind _box (Variables|Default|GetBox))
  (Rendering|Debug|DrawDebugBox (Transformation|GetWorldLocation _box) (Components|Box|GetScaledBoxExtent _box) "(R=1.000000,G=0.297447,B=0.080384,A=1.000000)" (Transformation|GetWorldRotation _box) NewParam 1e+01))

(fn CheckLaneEmpty
  (params (StartDist :type Float%20%28double-precision%29) (EndDist :type Float%20%28double-precision%29))
  (LocalVariables|SetStart (+ (Spline|GetLocationatDistanceAlongSpline (Variables|Default|GetSpline) StartDist "World") (LocalVariables|GetHeight)))
  (LocalVariables|SetEnd (+ (Spline|GetLocationatDistanceAlongSpline (Variables|Default|GetSpline) EndDist "World") (LocalVariables|GetHeight)))
  (bind _outhits (Class|KismetSystemLibrary|LineTraceMultiforObjects (LocalVariables|GetStart) (LocalVariables|GetEnd) (Utilities|Array|MakeArray "ObjectTypeQuery1" "ObjectTypeQuery2") false 0 "None" false))
  (for _array_element _outhits
    (if (.bBlockingHit (Collision|BreakHitResult _array_element))
      (if (>= (Utilities|Array|Length (Actor|GetComponentsByClass (.HitActor (Collision|BreakHitResult _array_element)) "/SimpleTrafficSim/Blueprint/SimpleTrafficSim/Blueprints/BPC_SimMovement.BPC_SimMovement_C")) 1)
        (return false))))
  (return true))