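; Traffic spawner actor that periodically creates cars for the simple traffic simulation, up to a count cap.
; At BeginPlay it box-traces forward to cache nearby BP_SplineLane actors as candidate lanes and starts a looping spawn timer.
; When its box is clear, it spawns a BP_CarMesh at its arrow with a random type and starting lane.
; Each car's BPC_SimMovement receives randomized speed and throttle plus a stop-time limit.
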(event Custom|Spawn
  (if (and (Variables|Default|GetEnableSpawn) (< (Variables|Default|GetSpawnNum) (Variables|Default|GetMaxNum)))
    (if (== (Utilities|Array|Length (Collision|GetOverlappingActors (Variables|Default|GetBox) (Variables|Default|GetClass%20Filter) :!class /Script/Engine.PrimitiveComponent)) 0)
      (CallFunction|RandomSpawn)
      (Math|Integer|IncrementInt (Variables|Default|GetSpawnNum)))))

(event Custom|Test
  (for _array_element (Collision|GetOverlappingActors (Variables|Default|GetBox) "/SimpleTrafficSim/Blueprint/SimpleTrafficSim/Blueprints/RoadSpline/BP_SplineLane.BP_SplineLane_C" :!class /Script/Engine.PrimitiveComponent)
    (Class|DimensioBPLibrary|PrintLog (Utilities|GetDisplayName _array_element))))

(event EventBeginPlay
  (Utilities|Time|SetTimerbyEvent (delegate Custom|Spawn) (Variables|Default|GetLoopTime) true)
  (CallFunction|DetectLanes))

(event Collision|EventActorBeginOverlap
  (params (OtherActor :type Actor%20Object%20Reference)))

(fn ConstructionScript)

(fn RandomSpawn
  (bind _returnvalue (Math|Random|RandomFloatinRange 5e+01 5.5e+02))
  (bind _returnvalue_2 (+ 9e+02 _returnvalue))
  (bind _returnvalue_3 (Game|SpawnActorfromClass "/SimpleTrafficSim/Blueprint/SimpleTrafficSim/Blueprints/BP_CarMesh.BP_CarMesh_C" (Transformation|GetWorldTransform (Variables|Default|GetArrow)) "Undefined" 0 (Math|Random|RandomInteger 25) (Actor|GetComponentbyClass (.OutItem (Utilities|Array|Random (Variables|Default|GetNexLanes))) "/Script/Engine.SplineComponent") false 0))
  (Utilities|IsValid _returnvalue_3
    (:Is%20Valid
      (Default|Autobots _returnvalue_3 (Variables|Default|GetAutobot))
      (EventDispatchers|BindEventtoNotifyVehicleHasDestroyed _returnvalue_3 (EventDispatchers|CreateEvent :!event IncreaseSpawnNum))
      (Default|InitSpeed (Actor|GetComponentbyClass _returnvalue_3 "/SimpleTrafficSim/Blueprint/SimpleTrafficSim/Blueprints/BPC_SimMovement.BPC_SimMovement_C") _returnvalue_2 (/ _returnvalue_2 3e+01))
      (Variables|/SimpleTrafficSim/Blueprint/SimpleTrafficSim/Blueprints/BPC_SimMovement.BPC_SimMovement_C|SetMaxStopTime (Actor|GetComponentbyClass _returnvalue_3 "/SimpleTrafficSim/Blueprint/SimpleTrafficSim/Blueprints/BPC_SimMovement.BPC_SimMovement_C") (Variables|Default|GetMax%20Stop%20Time)))
    (:Is%20Not%20Valid
      (Class|DimensioBPLibrary|PrintLog "Jsut Spawned! But Be Invalid!"))))

(fn BPSpawnCarAutoGenFunc
  (params (CarID :type Integer) (Car :type %20Object%20Reference)))

(fn CrowdCheck)

(fn IncreaseSpawnNum
  (Math|Integer|IncrementInt (Variables|Default|GetMaxNum)))

(fn DetectLanes
  (bind _returnvalue (Transformation|GetActorLocation))
  (bind _box (Variables|Default|GetBox))
  (bind _returnvalue_2 (Components|Box|GetScaledBoxExtent _box))
  (Utilities|Array|Clear (Variables|Default|GetNexLanes))
  (bind _outhits (Class|KismetSystemLibrary|BoxTraceMultiforObjects _returnvalue (+ _returnvalue (* (Transformation|GetActorForwardVector) (* (.Z (Math|Vector|BreakVector _returnvalue_2)) 4.0))) (/ _returnvalue_2 1.0) (Transformation|GetWorldRotation (Variables|Default|GetBox)) (Utilities|Array|MakeArray "ObjectTypeQuery1") false 0 "ForDuration" true))
  (for _array_element _outhits
    (bind _asbp_spline_lane (Utilities|Casting|CastToBP_SplineLane (.HitActor (Collision|BreakHitResult _array_element))))
    (Utilities|Array|Add (Variables|Default|GetNexLanes) _asbp_spline_lane)))