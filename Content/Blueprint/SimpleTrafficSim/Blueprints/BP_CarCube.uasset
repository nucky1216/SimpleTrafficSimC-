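; BP_CarCube is a traffic-sim car that exercises BPCSimMovement with simulated location input.
; A looping timer, toggled by SpaceBar, steps along SplinePath and sends randomly jittered points to the component, drawing separately randomized debug points.
; Tick pushes changed friction and SOD tuning (frequency, Z drag, R delay) into the component.
; Construction configures auto-drive and scales CarBox from the static mesh's bounds.
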(event Custom|Fake%20Sender
  (bind _gaptime (Variables|SODTest|GetGapTime))
  (bind _splinepath (Variables|SODTest|GetSplinePath))
  (bind _spline (Variables|/SimpleTrafficSim/Blueprint/SimpleTrafficSim/Blueprints/RoadSpline/BP_SplineDebug.BP_SplineDebug_C|GetSpline _splinepath))
  (bind _output_get (Variables|SODTest|SetDistAlongSpline (Math|Float|%(Float) (+ (Variables|SODTest|GetDistAlongSpline) (Variables|SODTest|GetGap%20Distance)) (Spline|GetSplineLength _spline))))
  (Default|RecieveLocInput (Variables|Default|GetBPC_SimMovement) (Math|Transform|MakeTransform (+ (* (Spline|GetDirectionatDistanceAlongSpline _spline _output_get "World") (Math|Random|RandomFloatinRange 0.0 2e+01)) (* (Class|SplineComponent|GetRightVectoratDistanceAlongSpline _spline _output_get "World") (Math|Random|RandomFloatinRange -2e+01 2e+01)) (Spline|GetLocationatDistanceAlongSpline _spline _output_get "World"))) _gaptime true)
  (Rendering|Debug|DrawDebugPoint (+ (* (Spline|GetDirectionatDistanceAlongSpline _spline _output_get "World") (Math|Random|RandomFloatinRange 0.0 2e+01)) (* (Class|SplineComponent|GetRightVectoratDistanceAlongSpline _spline _output_get "World") (Math|Random|RandomFloatinRange -2e+01 2e+01)) (Spline|GetLocationatDistanceAlongSpline _spline _output_get "World")) 2e+01 "(R=0.000000,G=1.000000,B=0.000000,A=1.000000)" _gaptime))

(event Custom|CustomEvent
  (bind _returnvalue (AddComponent|AddBillboardComponent true (Math|Transform|MakeTransform (/ (+ (Transformation|GetWorldLocation (Variables|Default|GetCarBox)) (Transformation|GetWorldLocation (Variables|Default|GetSphere)) (Transformation|GetWorldLocation (Variables|Default|GetSphere1))) 3.0) "0, 0, 0" "5.000000,5.000000,5.000000"))))

(event EventBeginPlay
  (bind _returnvalue (Utilities|Time|SetTimerbyEvent (delegate Custom|Fake%20Sender) (Variables|SODTest|GetGapTime) true))
  (bind _output_get (Variables|Default|SetTimer _returnvalue))
  (Utilities|Time|PauseTimerbyHandle _output_get))

(event EventTick
  (params (DeltaSeconds :type Float%20%28single-precision%29))
  (bind _in_zdrag (Variables|Default|GetIn%20ZDrag))
  (bind _in_rdelay (Variables|Default|GetIn%20RDelay))
  (bind _bpc_simmovement (Variables|Default|GetBPC_SimMovement))
  (bind _in_frac (Variables|Default|GetIn%20Frac))
  (bind _bpc_simmovement_2 (Variables|Default|GetBPC_SimMovement))
  (bind _in_freq (Variables|Default|GetIn%20Freq))
  (bind _returnvalue (Utilities|IsValid _bpc_simmovement))
  (bind _returnvalue_2 (Components|Activation|IsActive _bpc_simmovement))
  (bind _returnvalue_3 (Utilities|String|ToString(Boolean) _returnvalue))
  (bind _returnvalue_4 (Utilities|String|ToString(Boolean) _returnvalue_2))
  (bind _returnvalue_5 (Utilities|String|Append "BPC Valid:" _returnvalue_3 " Active :" _returnvalue_4))
  (Utilities|FlowControl|Sequence
    (:then_0
      (if (!= _in_frac (Variables|Default|GetFrac))
        (bind _output_get (Variables|Default|SetFrac _in_frac))
        (Class|DimensioBPLibrary|PrintLog _returnvalue_5)
        (Variables|/SimpleTrafficSim/Blueprint/SimpleTrafficSim/Blueprints/BPC_SimMovement.BPC_SimMovement_C|SetFriction _bpc_simmovement_2 _output_get)))
    (:then_1
      (if (Math|Boolean|ORBoolean (!= _in_freq (Variables|Default|GetFreq)) (!= _in_zdrag (Variables|Default|GetZDrag)) (!= _in_rdelay (Variables|Default|GetRDelay)))
        (bind _output_get_2 (Variables|Default|SetFreq _in_freq))
        (bind _output_get_3 (Variables|Default|SetZDrag _in_zdrag))
        (bind _output_get_4 (Variables|Default|SetRDelay _in_rdelay))
        (Class|DimensioBPLibrary|PrintLog _returnvalue_5)
        (Default|AdjustSOD _bpc_simmovement_2 _output_get_2 _output_get_3 _output_get_4)))))

(event Input|KeyboardEvents|SpaceBar
  (params (Key :type Key%20Structure))
  (bind _timer (Variables|Default|GetTimer))
  (:Pressed
    (Utilities|FlowControl|FlipFlop
      (:A
        (Utilities|Time|UnpauseTimerbyHandle _timer))
      (:B
        (Utilities|Time|PauseTimerbyHandle _timer)))))

(fn ConstructionScript
  (bind _staticmesh (Variables|Default|GetStaticMesh))
  (bind _staticmesh_2 (Variables|/Script/Engine.StaticMeshComponent|GetStaticMesh _staticmesh))
  (bind _returnvalue (StaticMesh|GetBoundingBox _staticmesh_2))
  (bind (_min _max) (Utilities|Struct|BreakBox _returnvalue))
  (Default|ConfigAutoDriveParms (Variables|Default|GetBPC_SimMovement) (Variables|Default|GetAuto%20Drive) (Variables|Default|GetCarBox) 35.0 1e+01)
  (Transformation|SetWorldScale3D (Variables|Default|GetCarBox) (/ (- _max _min) 1e+02)))